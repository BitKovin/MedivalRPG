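; Horse character with momentum-style movement, driven by forward and turn input events.
; Forward input raises a stored throttle that feeds movement along the facing direction each tick and eases back to zero when input drops, more slowly in reverse.
; Turn input yaws the actor directly, with steering flipped while backing up, and RunProgress blends max walk speed.
; Reins and saddle follow the body mesh's pose through master pose components.
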(event `Key|LeftShift`
  (params (Key :type "Key Structure")))

(event `MoveRightInput`
  (params (`Axis Value` :type "Float (double-precision)"))
  (bind (_returnvalue_roll _returnvalue_pitch _returnvalue_yaw) (`KismetMathLibrary.BreakRotator` (`self.K2_GetActorRotation`)))
  (set `self.RotatingVel` (* `Axis Value` (`self.RotationSpeed`)))
  (`self.K2_SetActorRotation` (`KismetMathLibrary.MakeRotator` 0.0 0.0 (+ (* (`self.RotationSpeed`) (`GameplayStatics.GetWorldDeltaSeconds`) `Axis Value`) _returnvalue_yaw))))

(event `self.ReceiveTick`
  (params (DeltaSeconds :type "Float (single-precision)"))
  (bind _forwardinput (`self.ForwardInput`))
  (set `self.RotationSpeed` (`KismetMathLibrary.SelectFloat` -90.0 90.0 (< (`self.ForwardInput`) 0.0)))
  (set `CharacterMovementComponent.MaxWalkSpeed` (`KismetMathLibrary.Lerp` 180.0 1000.0 (`self.RunProgress`)) (`self.CharacterMovement`))
  (`self.AddMovementInput` (`KismetMathLibrary.GetForwardVector` (`self.K2_GetActorRotation`)) (`self.ForwardInput`))
  (if (`self.NotMoving`)
    (if (> _forwardinput 0.0)
      (set `self.ForwardInput` (`KismetMathLibrary.FClamp` (- _forwardinput (* (`GameplayStatics.GetWorldDeltaSeconds`) 1.0))))
      (else
        (set `self.ForwardInput` (`KismetMathLibrary.FClamp` (+ (`self.ForwardInput`) (* (`GameplayStatics.GetWorldDeltaSeconds`) 0.5)) -1.0 0.0))))))

(event `MoveForwardInput`
  (params (`Axis Value` :type "Float (double-precision)"))
  (if (or (and (>= `Axis Value` (`self.ForwardInput`)) (> `Axis Value` 0.0) (>= (`self.ForwardInput`) 0.0)) (and (<= `Axis Value` 0.0) (< `Axis Value` (`self.ForwardInput`)) (<= (`self.ForwardInput`) 0.0)))
    (set `self.ForwardInput` `Axis Value`)
    (set `self.NotMoving` false)
    (else
      (set `self.NotMoving` true))))

(fn `UserConstructionScript`
  (`SkinnedMeshComponent.SetLeaderPoseComponent` (`self.Reins`) (`self.Mesh`) false)
  (`SkinnedMeshComponent.SetLeaderPoseComponent` (`self.Saddle`) (`self.Mesh`) false))