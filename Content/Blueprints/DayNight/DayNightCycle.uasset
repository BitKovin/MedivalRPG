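; Day/night cycle actor that advances a 24-hour clock on Tick, one in-game hour per 30 seconds of real time.
; Each update samples float curves at the wrapped time to set the Directional Light's pitch and its Sky Light's intensity.
; It also refreshes the BP_Sky_Sphere material to follow the sun, looking up both level actors by class every update.
; The construction script runs the same update, so the lighting previews in the editor.
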(event `UpdateTime`
  (bind _returnvalue (mod (`self.Time`) 24.0))
  (bind _returnvalue_2 (`GameplayStatics.GetActorOfClass` "/Engine/EngineSky/BP_Sky_Sphere.BP_Sky_Sphere_C"))
  (set `/Engine/EngineSky/BP_Sky_Sphere.Refresh material` true _returnvalue_2)
  (`/Engine/EngineSky/BP_Sky_Sphere.RefreshMaterial` _returnvalue_2)
  (bind _returnvalue_3 (`GameplayStatics.GetActorOfClass` "/Script/Engine.DirectionalLight"))
  (`self.K2_SetActorRotation` _returnvalue_3 (`KismetMathLibrary.MakeRotator` 10.0 (`CurveFloat.GetFloatValue` (`self.Rotation`) _returnvalue) 20.0) false)
  (`SkyLightComponent.SetIntensity` (`self.SkyLight`) (`CurveFloat.GetFloatValue` (`self.Rotation_0`) _returnvalue)))

(event `self.ReceiveTick`
  (params (DeltaSeconds :type "Float (single-precision)"))
  (`self.UpdateTime`)
  (set `self.Time` (+ (`self.Time`) (/ (`GameplayStatics.GetWorldDeltaSeconds`) 30.0))))

(fn `UserConstructionScript`
  (`self.UpdateTime`))