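; Sword actor that assembles a seeded random variant from preplaced blade, crossguard, hilt and pommel components.
; The construction script calls GenerateSwordFunc, which selects one component per part and makes it visible, without hiding the others.
; Each pick starts a fresh random stream from the same Seed, so results are repeatable but correlated: blade and pommel share an index, as do crossguard and hilt.
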(fn `GenerateSwordFunc`
  (`SceneComponent.SetVisibility` (select `int` (`KismetMathLibrary.RandomIntegerInRangeFromStream` 0 2 (`KismetMathLibrary.MakeRandomStream` (`self.Seed`))) :`0` (`self.sword_blade_03`) :`1` (`self.sword_blade_04`) :`2` (`self.sword_blade_05`) :!type "SceneComponent Object Reference") true false)
  (`SceneComponent.SetVisibility` (select `int` (`KismetMathLibrary.RandomIntegerInRangeFromStream` 0 4 (`KismetMathLibrary.MakeRandomStream` (`self.Seed`))) :`0` (`self.sword_crossguard_02`) :`1` (`self.Sword_crossguard_01`) :`2` (`self.sword_crossguard_05`) :`3` (`self.sword_crossguard_04`) :`4` (`self.Sword_crossguard_08`) :!type "SceneComponent Object Reference") true false)
  (`SceneComponent.SetVisibility` (select `int` (`KismetMathLibrary.RandomIntegerInRangeFromStream` 0 4 (`KismetMathLibrary.MakeRandomStream` (`self.Seed`))) :`0` (`self.Sword_hilt_011`) :`1` (`self.sword_hilt_02`) :`2` (`self.sword_hilt_04`) :`3` (`self.Sword_hilt_01`) :`4` (`self.Sword_hilt_010`) :!type "SceneComponent Object Reference") true false)
  (`SceneComponent.SetVisibility` (select `int` (`KismetMathLibrary.RandomIntegerInRangeFromStream` 0 2 (`KismetMathLibrary.MakeRandomStream` (`self.Seed`))) :`0` (`self.Sword_pommel_01`) :`1` (`self.Sword_pommel_08`) :`2` (`self.Sword_pommel_05`) :!type "SceneComponent Object Reference") true false))

(fn `UserConstructionScript`
  (`self.GenerateSwordFunc`))