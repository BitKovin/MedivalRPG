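; Behavior tree task that makes an NPC stop blocking when the block is no longer needed.
; It gets the controlled BP_NPC from the AI controller and calls UnBlock if its Target is invalid or that target's Aim is below a fixed threshold.
; The task always finishes with success, even when the casts fail or the NPC keeps blocking.
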(event `self.ReceiveExecute`
  (params (OwnerActor :type "Actor Object Reference"))
  (bind _asaicontroller (cast `AIController` OwnerActor)
    (:`then`
      (bind _asbp_npc (cast `/Game/Blueprints/AI/BP_NPC` (`Controller.K2_GetPawn` _asaicontroller))
        (:`then`
          (bind _target (`/Game/Blueprints/AI/BP_NPC.Target` _asbp_npc))
          (`/Engine/EditorBlueprintResources/StandardMacros.IsValid` _target
            (:`Is Valid`
              (if (< (`/Game/MultiplayerFPSEngine/Blueprints/BP_PlayerBase.aim` _target) 0.5)
                (`/Game/MultiplayerFPSEngine/Blueprints/BP_PlayerBase.UnBlock` _asbp_npc :!label _label)))
            (:`Is Not Valid`
              (goto _label)))
          (`self.FinishExecute` true))
        (:`CastFailed`
          (`self.FinishExecute` true :!label _label_2))))
    (:`CastFailed`
      (goto _label_2))))