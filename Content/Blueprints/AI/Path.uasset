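; AI path actor that defines a route with a spline and exposes lookups between spline keys and world locations.
; The construction script sizes the WaitAfterKeys array to the spline point count and rebuilds index text labels at each point as an editing aid.
; BeginPlay destroys those labels.
; GetLocation wraps keys by the point count for looping, and GetNearestKey returns the key closest to a world location.
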(event `self.ReceiveBeginPlay`
  (for _array_element (`self.TRC`)
    (`ActorComponent.K2_DestroyComponent` _array_element)))

(fn `GetLocation`
  (params (Key :type "Float (double-precision)"))
  (returns (Location :type "Vector Structure"))
  (bind _spline (`self.Spline`))
  (return (`SplineComponent.GetLocationAtSplineInputKey` _spline (mod Key (`KismetMathLibrary.Conv_IntToDouble` (`SplineComponent.GetNumberOfSplinePoints` _spline))) "World")))

(fn `GetNearest Key`
  (params (Location :type "Vector Structure"))
  (returns (Key :type "Float (double-precision)"))
  (return (`SplineComponent.FindInputKeyClosestToWorldLocation` (`self.Spline`) Location)))

(fn `UserConstructionScript`
  (bind _spline (`self.Spline`))
  (bind _waitafterkeys (`self.WaitAfterKeys`))
  (bind _returnvalue (`SplineComponent.GetNumberOfSplinePoints` (`self.Spline`)))
  (`KismetArrayLibrary.Array_Set` _waitafterkeys _returnvalue 0.0 true)
  (`KismetArrayLibrary.Array_Remove` _waitafterkeys _returnvalue)
  (for _array_element (`self.TRC`)
    (`ActorComponent.K2_DestroyComponent` _array_element))
  (for _index (range (`SplineComponent.GetNumberOfSplinePoints` (`self.Spline`)))
    (bind _returnvalue_2 (`AddComponent|NODE_AddTextRenderComponent-0` :`RelativeTransform` (`KismetMathLibrary.MakeTransform` (`SplineComponent.GetLocationAtSplineInputKey` _spline (mod (`KismetMathLibrary.Conv_IntToDouble` _index) (`KismetMathLibrary.Conv_IntToDouble` (`SplineComponent.GetNumberOfSplinePoints` _spline))) "Local") (struct :`Pitch` 90.0))))
    (`KismetArrayLibrary.Array_Add` (`self.TRC`) _returnvalue_2)
    (`TextRenderComponent.K2_SetText` _returnvalue_2 (`KismetTextLibrary.Conv_IntToText` _index))))