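; BP_NPC_Citizen is a citizen NPC that plays idle activity montages for washing windows and relaxing its legs.
; Custom start events play each montage through its own DoOnce, so repeated calls do not restart it.
; The matching end events reset that DoOnce; only the window-washing end also stops its montage.
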(event `WashWindows`
  (`/Engine/EditorBlueprintResources/StandardMacros.DoOnce` false :!label _label
    (:`Completed`
      (`self.PlayAnimMontage` "/Game/Animations/NPC/Montages/Anim_Washing_Window_Montage.Anim_Washing_Window_Montage"))))

(event `WashWindowsEnd`
  (`self.StopAnimMontage` "/Game/Animations/NPC/Montages/Anim_Washing_Window_Montage.Anim_Washing_Window_Montage")
  (goto _label :!via `Reset`))

(event `LegsRelax`
  (`/Engine/EditorBlueprintResources/StandardMacros.DoOnce` false :!label _label_2
    (:`Completed`
      (`self.PlayAnimMontage` "/Game/Animations/NPC/Montages/Anim_Legs_Relax_Montage.Anim_Legs_Relax_Montage"))))

(event `LegsRelaxEnd`
  (goto _label_2 :!via `Reset`))

(fn `UserConstructionScript`
  (`parent.UserConstructionScript`))