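; Behavior tree task that gives an AI-controlled BP_NPC a random chance to block.
; On execute it gets the pawn from the owning AIController and calls TryBlock when two random booleans are both true, roughly a one-in-four chance.
; The task finishes immediately with success in every case, including a missed roll or failed cast.
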(event `self.ReceiveExecute`
  (params (OwnerActor :type "Actor Object Reference"))
  (bind _asaicontroller (cast `AIController` OwnerActor)
    (:`then`
      (bind _asbp_npc (cast `/Game/Blueprints/AI/BP_NPC` (`Controller.K2_GetPawn` _asaicontroller))
        (:`then`
          (if (`KismetMathLibrary.Conv_IntToBool` (* (`KismetMathLibrary.Conv_BoolToInt` (`KismetMathLibrary.RandomBool`)) (`KismetMathLibrary.Conv_BoolToInt` (`KismetMathLibrary.RandomBool`))))
            (`/Game/MultiplayerFPSEngine/Blueprints/BP_PlayerBase.TryBlock` _asbp_npc)
            (`self.FinishExecute` true)
            (else
              (`self.FinishExecute` true :!label _label))))
        (:`CastFailed`
          (goto _label))))
    (:`CastFailed`
      (goto _label))))