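; Guard NPC that spawns with a sword in its auto-slot list and picks a threat through pawn sensing when it has no target.
; Guards outside the default NPC type target sighted player-base pawns of other non-default types, or flee them if slot 0 is empty.
; Default-type guards react to same-type NPCs, targeting what they flee from when armed, or copying a fellow guard's target.
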(event `self.ReceiveBeginPlay`
  (bind _returnvalue (`|SpawnActorFromClass` "/Game/Inventory/Items/BP_Sword.BP_Sword_C" (`KismetMathLibrary.MakeTransform` (0.0 0.0 0.0)) "Undefined" "OverrideRootScale" null null null null))
  (`KismetArrayLibrary.Array_Set` (`self.AutoAddToSlots`) 0 _returnvalue true)
  (`parent.ReceiveBeginPlay`))

(event `self.PawnSensing.OnSeePawn`
  (params (Pawn :type "Pawn Object Reference"))
  (`/Engine/EditorBlueprintResources/StandardMacros.IsValid` (`self.Target`)
    (:`Is Not Valid`
      (if (`|EnumInequality` (`self.NPCType`) "NewEnumerator0")
        (bind _asbp_player_base (cast `/Game/MultiplayerFPSEngine/Blueprints/BP_PlayerBase` Pawn))
        (bind _npctype (`/Game/MultiplayerFPSEngine/Blueprints/BP_PlayerBase.NPCType` _asbp_player_base))
        (if (and (`|EnumInequality` _npctype "NewEnumerator0") (`|EnumInequality` _npctype (`self.NPCType`)))
          (`/Engine/EditorBlueprintResources/StandardMacros.IsValid` (`|GetArrayItem` (`self.Slots`))
            (:`Is Valid`
              (set `self.Target` _asbp_player_base))
            (:`Is Not Valid`
              (set `self.RunAwayFrom` _asbp_player_base))))
        (else
          (bind _asbp_npc (cast `/Game/Blueprints/AI/BP_NPC` Pawn))
          (if (`|EnumEquality` (`/Game/MultiplayerFPSEngine/Blueprints/BP_PlayerBase.NPCType` _asbp_npc) "NewEnumerator0")
            (bind _runawayfrom (`/Game/Blueprints/AI/BP_NPC.RunAwayFrom` _asbp_npc))
            (`/Engine/EditorBlueprintResources/StandardMacros.IsValid` _runawayfrom
              (:`Is Valid`
                (`/Engine/EditorBlueprintResources/StandardMacros.IsValid` (`|GetArrayItem` (`self.Slots`))
                  (:`Is Valid`
                    (set `self.Target` _runawayfrom))))
              (:`Is Not Valid`
                (bind _asbp_npc_guard (cast `/Game/Blueprints/AI/Guard/BP_NPC_Guard` _asbp_npc))
                (bind _target (`/Game/Blueprints/AI/BP_NPC.Target` _asbp_npc_guard))
                (`/Engine/EditorBlueprintResources/StandardMacros.IsValid` _target
                  (:`Is Valid`
                    (set `self.Target` _target)))))))))))

(fn `UserConstructionScript`
  (`parent.UserConstructionScript`))