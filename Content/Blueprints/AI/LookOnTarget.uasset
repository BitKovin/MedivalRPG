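; Behavior tree task that turns a BP_NPC to face its current Target.
; On execute it stores the pawn's starting rotation, failing if the Target is invalid.
; Tick then lerps by shortest path toward the look-at yaw, recomputed each frame, over about a sixth of a second.
; It finishes successfully once the turn completes and resets its timer.
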(event `self.ReceiveExecute`
  (params (OwnerActor :type "Actor Object Reference"))
  (bind _asaicontroller (cast `AIController` OwnerActor)
    (:`then`
      (bind _asbp_npc (cast `/Game/Blueprints/AI/BP_NPC` (`Controller.K2_GetPawn` _asaicontroller)))
      (`/Engine/EditorBlueprintResources/StandardMacros.IsValid` (`/Game/Blueprints/AI/BP_NPC.Target` _asbp_npc)
        (:`Is Valid`
          (set `self.OldRotation` (`Actor.K2_GetActorRotation` _asbp_npc)))
        (:`Is Not Valid`
          (`self.FinishExecute` false))))
    (:`CastFailed`
      (`self.FinishExecute` true))))

(event `self.ReceiveTick`
  (params (OwnerActor :type "Actor Object Reference") (DeltaSeconds :type "Float (single-precision)"))
  (bind _returnvalue (`KismetMathLibrary.FClamp` (* (`self.Time`) 6.0)))
  (bind _target (`/Game/Blueprints/AI/BP_NPC.Target` (stale `self.ReceiveExecute` _asbp_npc)))
  (`/Engine/EditorBlueprintResources/StandardMacros.IsValid` _target
    (:`Is Valid`
      (set `self.Time` (+ (`self.Time`) DeltaSeconds))
      (`/Engine/EditorBlueprintResources/StandardMacros.IsValid` (stale `self.ReceiveExecute` _asbp_npc)
        (:`Is Valid`
          (bind (_returnvalue_roll _returnvalue_pitch _returnvalue_yaw) (`KismetMathLibrary.BreakRotator` (`KismetMathLibrary.FindLookAtRotation` (`Actor.K2_GetActorLocation` (stale `self.ReceiveExecute` _asbp_npc)) (`Actor.K2_GetActorLocation` _target))))
          (`Actor.K2_SetActorRotation` (stale `self.ReceiveExecute` _asbp_npc) (`KismetMathLibrary.RLerp` (`self.OldRotation`) (`KismetMathLibrary.MakeRotator` 0.0 0.0 _returnvalue_yaw) _returnvalue true) false)
          (if (== _returnvalue 1.0)
            (`self.FinishExecute` true)
            (set `self.Time` 0.0)))))))