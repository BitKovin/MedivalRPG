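; AI-driven NPC character that patrols waypoint paths, optionally scheduled by day/night hour, and fights or flees threats.
; Sight and damage set Target or RunAwayFrom based on NPC type and whether slot 0 is filled.
; Tick feeds that state to a behavior tree blackboard, with a line-traced helper actor marking the escape point, and pauses this during mind control.
; Save hooks store and restore path, target, weapon and inventory, then restart the AI.
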(event `self.ReceiveBeginPlay`
  (`parent.ReceiveBeginPlay`)
  (bind _returnvalue (`GameplayStatics.GetActorOfClass` "/Game/Blueprints/DayNight/DayNightCycle.DayNightCycle_C"))
  (set `self.Time` _returnvalue)
  (bind _returnvalue_2 (`|SpawnActorFromClass` "/Game/Blueprints/AI/RunAwayPOint.RunAwayPOint_C" (`KismetMathLibrary.MakeTransform` (0.0 0.0 0.0)) "Undefined" "OverrideRootScale" null null))
  (set `self.RunAwayActor` _returnvalue_2)
  (`/Engine/EditorBlueprintResources/StandardMacros.IsValid` (`self.Path`)
    (:`Is Valid`
      (if (not (`self.TimeAttachedWaypoints`))
        (`self.FindFirstkey`)))
    (:`Is Not Valid`
      _))
  (for _array_element (`self.AutoAddToInventory`)
    (`/Game/Inventory/InventoryComponent.TryAddItem` (`self.InventoryComponent`) (`/Game/Inventory/BP_item.ItemObject` _array_element))
    (`self.K2_DestroyActor` _array_element))
  (for (_array_element_2 _array_index) (`self.AutoAddToSlots`)
    (`KismetArrayLibrary.Array_Set` (`/Game/Inventory/InventoryComponent.Slots` (`self.InventoryComponent`)) _array_index (`/Game/Inventory/BP_item.ItemObject` _array_element_2) true)
    (`/Game/Inventory/InventoryComponent.Update Slots` (`self.InventoryComponent`) (`KismetMathLibrary.Conv_IntToByte` _array_index))
    (`self.K2_DestroyActor` _array_element_2))
  (`|ExecutionSequence`
    (:`then_0`
      (if (`self.TimeAttachedWaypoints`)
        (bind _location (`/Game/Blueprints/AI/Path.GetLocation` (`self.Path`) (`KismetMathLibrary.Conv_IntToDouble` (`self.Key`))))
        (set `self.TargetPathPoint` _location)))
    (:`then_1`
      (bind _asaicontroller (cast `AIController` (`self.GetController`) :!label _label))
      (bind _blackboardcomponent (`AIController.UseBlackboard` _asaicontroller "/Game/Blueprints/AI/NewBlackboardData.NewBlackboardData"))
      (set `self.Blackboard Component` _blackboardcomponent)
      (`AIController.RunBehaviorTree` _asaicontroller "/Game/Blueprints/AI/TestBehaviorTree.TestBehaviorTree")
      (`self.PathUpdate`))))

(event `self.AfterDeath`
  (bind _asaicontroller (cast `AIController` (`self.GetController`)))
  (`BrainComponent.StopLogic` (`AIController.BrainComponent` _asaicontroller) "Died"))

(event `ReInitAi`
  (goto _label))

(event `Attack`
  (bind _weapon_bp (`self.Weapon_BP`))
  (`/Game/MultiplayerFPSEngine/Blueprints/Weapon/BP_Weapon.LMBPressed` _weapon_bp)
  (`/Game/MultiplayerFPSEngine/Blueprints/Weapon/BP_Weapon.LMBReleased` _weapon_bp))

(event `self.ReceiveTick`
  (params (DeltaSeconds :type "Float (single-precision)"))
  (bind _target (`self.Target`))
  (bind _blackboard_component (`self.Blackboard Component`))
  (`parent.ReceiveTick` DeltaSeconds)
  (`|ExecutionSequence`
    (:`then_0`
      (`self.MindControllUpdate`)
      (if (not (`self.mindControll`))
        (`self.UpdateRunAway`)
        (`self.UpdateCombat`)
        (`self.K2_SetActorLocation` (`self.RunAwayActor`) (`self.GetRunAwayLocation`) false true)
        (`self.PathUpdate`)
        (`BlackboardComponent.SetValueAsObject` (`self.Blackboard Component`) "RunAwayLocation" (`self.RunAwayActor`))
        (`BlackboardComponent.SetValueAsObject` (`self.Blackboard Component`) "RunAwayFrom" (`self.RunAwayFrom`))
        (`BlackboardComponent.SetValueAsBool` (`self.Blackboard Component`) "Talking" (`self.Talking`))
        (`BlackboardComponent.SetValueAsBool` (`self.Blackboard Component`) "RestartWalk" (`self.RestartWalk`))
        (`BlackboardComponent.SetValueAsBool` (`self.Blackboard Component`) "MindControll" (`self.mindControll`))
        (`BlackboardComponent.SetValueAsBool` (`self.Blackboard Component`) "Stun" (`self.stun`))
        (`BlackboardComponent.SetValueAsObject` (`self.Blackboard Component`) "Target" _target)
        (`/Engine/EditorBlueprintResources/StandardMacros.IsValid` _target
          (:`Is Valid`
            (`BlackboardComponent.SetValueAsBool` _blackboard_component "TargetIsBlocking" (> (`/Game/MultiplayerFPSEngine/Blueprints/BP_PlayerBase.aim` (`self.Target`)) 0.0))
            (if (<= (`/Game/MultiplayerFPSEngine/Blueprints/BP_PlayerBase.health` (`self.Target`)) 0.0)
              (`KismetSystemLibrary.Delay` 1.0 :!label _label_2)
              (`self.ChangeSlot` 2)
              (elif (not (`AnimInstance.Montage_IsPlaying` (`SkeletalMeshComponent.GetAnimInstance` (`self.Mesh`)) "/Game/Animations/Sword/Sword1h_Hit_Torso_Front_Montage.Sword1h_Hit_Torso_Front_Montage"))
                (`self.ChangeSlot` 0))))
          (:`Is Not Valid`
            (`BlackboardComponent.SetValueAsBool` _blackboard_component "TargetIsBlocking" false)
            (goto _label_2)))))
    (:`then_1`
      (if (<= (`self.health`) 0.0)
        (`/Engine/EditorBlueprintResources/StandardMacros.DoOnce` false :!label _label_3
          (:`Completed`
            (`KismetSystemLibrary.Delay` 5.0)
            (set `self.Target` null)
            (set `self.RunAwayFrom` null)))
        (else
          (goto _label_3 :!via `Reset`))))))

(event `self.DamagedBy`
  (params (character :type "/Game/MultiplayerFPSEngine/Blueprints/BP_PlayerBase Object Reference"))
  (bind _npctype (`/Game/MultiplayerFPSEngine/Blueprints/BP_PlayerBase.NPCType` character))
  (`KismetSystemLibrary.PrintString` "Hello")
  (`/Engine/EditorBlueprintResources/StandardMacros.IsValid` (`self.Target`)
    (:`Is Not Valid`
      (if (!= character self)
        (if (or (`|EnumEquality` (`self.NPCType`) "NewEnumerator0") (and (`|EnumInequality` _npctype "NewEnumerator0") (`|EnumInequality` (`self.NPCType`) _npctype)))
          (`/Engine/EditorBlueprintResources/StandardMacros.IsValid` (`|GetArrayItem` (`self.Slots`))
            (:`Is Valid`
              (set `self.Target` character))
            (:`Is Not Valid`
              (set `self.RunAwayFrom` character))))))))

(event `UpdateCombat`
  (bind _target (`self.Target`))
  (bind _returnvalue (`self.GetDistanceTo` _target self))
  (`KismetSystemLibrary.Delay` 0.2)
  (`/Engine/EditorBlueprintResources/StandardMacros.IsValid` _target
    (:`Is Valid`
      (if (<= (`/Game/MultiplayerFPSEngine/Blueprints/BP_PlayerBase.health` (`self.Target`)) 0.0)
        (set `self.Target` null)
        (elif (> _returnvalue 4500.0)
          (set `self.Target` null)
          (elif (> _returnvalue 300.0)
            (set `self.W` true)
            (set `self.Shift` true)
            (else
              (set `self.W` false)
              (set `self.Shift` false))))))))

(event `self.PawnSensing.OnSeePawn`
  (params (Pawn :type "Pawn Object Reference"))
  (`/Engine/EditorBlueprintResources/StandardMacros.IsValid` (`self.Target`)
    (:`Is Not Valid`
      (if (`self.isMonster`)
        (bind _asbp_player_base (cast `/Game/MultiplayerFPSEngine/Blueprints/BP_PlayerBase` Pawn))
        (set `self.Target` _asbp_player_base)
        (elif (`|EnumInequality` (`self.NPCType`) "NewEnumerator0")
          (bind _asbp_player_base_2 (cast `/Game/MultiplayerFPSEngine/Blueprints/BP_PlayerBase` Pawn))
          (bind _npctype (`/Game/MultiplayerFPSEngine/Blueprints/BP_PlayerBase.NPCType` _asbp_player_base_2))
          (if (and (`|EnumInequality` _npctype "NewEnumerator0") (`|EnumInequality` _npctype (`self.NPCType`)))
            (`/Engine/EditorBlueprintResources/StandardMacros.IsValid` (`|GetArrayItem` (`self.Slots`))
              (:`Is Valid`
                (set `self.Target` _asbp_player_base_2))
              (:`Is Not Valid`
                (set `self.RunAwayFrom` _asbp_player_base_2))))
          (else
            (bind _asbp_npc (cast `/Game/Blueprints/AI/BP_NPC` Pawn))
            (if (`|EnumEquality` (`/Game/MultiplayerFPSEngine/Blueprints/BP_PlayerBase.NPCType` _asbp_npc) "NewEnumerator0")
              (bind _runawayfrom (`/Game/Blueprints/AI/BP_NPC.RunAwayFrom` _asbp_npc))
              (`/Engine/EditorBlueprintResources/StandardMacros.IsValid` _runawayfrom
                (:`Is Valid`
                  (`/Engine/EditorBlueprintResources/StandardMacros.IsValid` (`|GetArrayItem` (`self.Slots`))
                    (:`Is Valid`
                      (set `self.Target` _runawayfrom))))))))))))

(event `ReachedPoint`
  (bind _keys (`/Game/Blueprints/AI/Path.Keys` (`self.Path`)))
  (bind (_output_waitafterreach _output_calleventafterreach _output_calleventaftermoveaway) (break `/Game/Blueprints/AI/WayPoint` (`|GetArrayItem` _keys (mod (`self.Key`) (`KismetArrayLibrary.Array_Length` _keys)))))
  (`Dialogue.CallFunctionByName` self _output_calleventafterreach)
  (if (> _output_waitafterreach 0.0)
    (`KismetSystemLibrary.Delay` _output_waitafterreach)
    (`Dialogue.CallFunctionByName` self _output_calleventaftermoveaway)
    (set `self.RestartWalk` false)
    (`self.GoToNextPoint`)
    (else
      (`self.GoToNextPoint`)
      (set `self.RestartWalk` false))))

(event `FindFirstkey`
  (bind _key (`/Game/Blueprints/AI/Path.GetNearest Key` (`self.Path`) (`self.K2_GetActorLocation`)))
  (set `self.Key` (+ (`KismetMathLibrary.FTrunc` _key) 1))
  (bind _location (`/Game/Blueprints/AI/Path.GetLocation` (`self.Path`) (`KismetMathLibrary.Conv_IntToDouble` (`self.Key`))))
  (set `self.TargetPathPoint` _location))

(event `GoToNextPoint`
  (bind _path (`self.Path`))
  (if (not (`self.TimeAttachedWaypoints`))
    (bind _output_get (set `self.Key` (+ (`self.Key`) 1)))
    (`/Engine/EditorBlueprintResources/StandardMacros.IsValid` _path
      (:`Is Valid`
        (bind _location (`/Game/Blueprints/AI/Path.GetLocation` _path (`KismetMathLibrary.Conv_IntToDouble` _output_get)))
        (set `self.TargetPathPoint` _location)
        (`self.PathUpdate`)))))

(event `EMSActorSaveInterface.ActorPreSave`
  (set `self.PathSave` (`|ConvertAsset` (`self.Path`)))
  (set `self.targetSave` (`|ConvertAsset` (`self.Target`)))
  (set `self.WeaponBpSave` (`|ConvertAsset` (`self.Weapon_BP`)))
  (for (_array_element _array_index) (`self.Slots`)
    (`KismetArrayLibrary.Array_Set` (`self.SlotsSave`) _array_index (`|ConvertAsset` _array_element) true))
  (for (_array_element_2 _array_index_2) (`/Game/Inventory/InventoryComponent.items` (`self.InventoryComponent`))
    (`KismetArrayLibrary.Array_Set` (`self.InventorySave`) _array_index_2 (`|ConvertAsset` _array_element_2) true))
  (for (_array_element_3 _array_index_3) (`/Game/Inventory/InventoryComponent.Slots` (`self.InventoryComponent`))
    (`KismetArrayLibrary.Array_Set` (`self.InventorySlotsSave`) _array_index_3 (`|ConvertAsset` _array_element_3) true)))

(event `MindControllUpdate`
  (if (== (`self.DefaultController`) (`self.GetController`))
    (set `CharacterMovementComponent.bOrientRotationToMovement` true (`self.CharacterMovement`))
    (set `self.bUseControllerRotationYaw` false)
    (set `self.mindControll` false)
    (`/Engine/EditorBlueprintResources/StandardMacros.DoOnce` true :!label _label_4
      (:`Completed`
        (`self.ReInitAi`)))
    (else
      (set `CharacterMovementComponent.bOrientRotationToMovement` false (`self.CharacterMovement`))
      (set `self.bUseControllerRotationYaw` true)
      (set `self.mindControll` true)
      (goto _label_4 :!via `Reset`))))

(event `UpdateRunAway`
  (bind _runawayfrom (`self.RunAwayFrom`))
  (bind _returnvalue (`KismetSystemLibrary.IsValid` (`self.RunAwayFrom`)))
  (`/Engine/EditorBlueprintResources/StandardMacros.IsValid` _runawayfrom
    (:`Is Valid`
      (`|ExecutionSequence`
        (:`then_0`
          (if (> (`self.GetDistanceTo` _runawayfrom self) 5000.0)
            (set `self.RunAwayFrom` null)))
        (:`then_1`
          (`/Engine/EditorBlueprintResources/StandardMacros.IsValid` (`self.Target`) :!label _label_5
            (:`Is Not Valid`
              (set `self.Shift` _returnvalue)
              (set `self.W` _returnvalue))))))
    (:`Is Not Valid`
      (goto _label_5))))

(event `PathUpdate`
  (bind _key (`self.Key`))
  (bind _keys (`/Game/Blueprints/AI/Path.Keys` (`self.Path`)))
  (bind _keys_2 (`/Game/Blueprints/AI/Path.Keys` (`self.Path`)))
  (bind (_value _returnvalue) (`BlueprintMapLibrary.Map_Find` (`self.TimeToPoints`) (`KismetMathLibrary.FTrunc` (mod (`/Game/Blueprints/DayNight/DayNightCycle.Time` (`self.Time`)) 24.0))))
  (bind (_output_waitafterreach _output_calleventafterreach _output_calleventaftermoveaway) (break `/Game/Blueprints/AI/WayPoint` (`|GetArrayItem` _keys (mod (`self.Key`) (`KismetArrayLibrary.Array_Length` _keys)))))
  (bind (_output_waitafterreach_2 _output_calleventafterreach_2 _output_calleventaftermoveaway_2 _output_lookonwhenreach _output_lookrotation) (break `/Game/Blueprints/AI/WayPoint` (`|GetArrayItem` _keys_2 (`KismetMathLibrary.FTrunc` (mod (`KismetMathLibrary.Conv_IntToDouble` _key) (`KismetMathLibrary.Conv_IntToDouble` (`KismetArrayLibrary.Array_Length` _keys_2)))))))
  (if (!= _key -1)
    (`/Engine/EditorBlueprintResources/StandardMacros.IsValid` (`self.Path`)
      (:`Is Valid`
        (set `self.LookAtRotation` _output_lookrotation)
        (`BlackboardComponent.SetValueAsVector` (`self.Blackboard Component`) "TargetPathPoint" (`self.TargetPathPoint`))
        (`BlackboardComponent.SetValueAsBool` (`self.Blackboard Component`) "LookOnWhenReach" _output_lookonwhenreach)
        (if (`self.TimeAttachedWaypoints`)
          (if _returnvalue
            (`Dialogue.CallFunctionByName` self _output_calleventaftermoveaway)
            (bind _output_get (set `self.Key` _value))
            (bind _location (`/Game/Blueprints/AI/Path.GetLocation` (`self.Path`) (`KismetMathLibrary.Conv_IntToDouble` _output_get)))
            (set `self.TargetPathPoint` _location)))))))

(event `EMSActorSaveInterface.ActorLoaded`
  (`EMSAsyncWait.AsyncWaitForOperation`
    (:`OnCompleted`
      (set `self.Path` (`|ConvertAsset` (`self.PathSave`)))
      (set `self.Weapon_BP` (`|ConvertAsset` (`self.WeaponBpSave`)))
      (set `self.Target` (`|ConvertAsset` (`self.targetSave`)))
      (for (_array_element _array_index) (`self.SlotsSave`)
        (`KismetArrayLibrary.Array_Set` (`self.Slots`) _array_index (`|ConvertAsset` _array_element) true))
      (for (_array_element_2 _array_index_2) (`self.InventorySave`)
        (`KismetArrayLibrary.Array_Set` (`/Game/Inventory/InventoryComponent.items` (`self.InventoryComponent`)) _array_index_2 (`|ConvertAsset` _array_element_2) true))
      (for (_array_element_3 _array_index_3) (`self.InventorySlotsSave`)
        (`KismetArrayLibrary.Array_Set` (`/Game/Inventory/InventoryComponent.Slots` (`self.InventoryComponent`)) _array_index_3 (`|ConvertAsset` _array_element_3) true))
      (set `self.Key` (- (`self.Key`) 1))
      (`self.GoToNextPoint`)
      (`KismetSystemLibrary.Delay` 0.0)
      (`self.ReInitAi`)
      (set `self.RestartWalk` true)
      (`KismetSystemLibrary.Delay` 0.5)
      (set `self.RestartWalk` false))))

(fn `ComponentsToSave`
  (returns (Components :type "Array of ActorComponent Object Reference"))
  (return (`|MakeArray` (`self.InventoryComponent`) :!type "ActorComponent Object Reference")))

(fn `GetRunAwayLocation`
  (returns (Location :type "Vector Structure"))
  (bind _returnvalue (+ (`self.K2_GetActorLocation`) (* (`KismetMathLibrary.GreaterGreater_VectorRotator` (`KismetMathLibrary.GetForwardVector` (`KismetMathLibrary.FindLookAtRotation` (`self.K2_GetActorLocation` (`self.RunAwayFrom`)) (`self.K2_GetActorLocation`))) (struct :`Yaw` 5.0)) 5000.0)))
  (`/Engine/EditorBlueprintResources/StandardMacros.IsValid` (`self.RunAwayFrom`)
    (:`Is Valid`
      (bind _outhit (`KismetSystemLibrary.LineTraceSingle` :`Start` (+ _returnvalue (0.0 0.0 10000.0)) :`End` (+ _returnvalue (0.0 0.0 -1000.0)) :`TraceChannel` "TraceTypeQuery1" :`DrawDebugType` "ForOneFrame" :`DrawTime` 0.1))
      (return (`.Location` (`GameplayStatics.BreakHitResult` _outhit))))
    (:`Is Not Valid`
      (return (+ (`self.K2_GetActorLocation`) (* (`KismetMathLibrary.GetForwardVector` (`self.K2_GetActorRotation`)) 1000.0))))))

(fn `UserConstructionScript`
  (`parent.UserConstructionScript`))