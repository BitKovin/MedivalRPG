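; Behavior tree task that smoothly turns a BP_NPC to the yaw stored in its LookAtRotation.
; On execute it caches the NPC's starting rotation, failing if no player character exists, though the player's position is not used.
; Tick lerps along the shortest path over half a second, then finishes successfully and resets its timer.
; A non-AI owner also reports success, while a failed NPC cast never finishes execution.
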(event `self.ReceiveExecute`
  (params (OwnerActor :type "Actor Object Reference"))
  (bind _asaicontroller (cast `AIController` OwnerActor)
    (:`then`
      (bind _asbp_npc (cast `/Game/Blueprints/AI/BP_NPC` (`Controller.K2_GetPawn` _asaicontroller)))
      (`/Engine/EditorBlueprintResources/StandardMacros.IsValid` (`GameplayStatics.GetPlayerCharacter` 0)
        (:`Is Valid`
          (set `self.OldRotation` (`Actor.K2_GetActorRotation` _asbp_npc)))
        (:`Is Not Valid`
          (`self.FinishExecute` false))))
    (:`CastFailed`
      (`self.FinishExecute` true))))

(event `self.ReceiveTick`
  (params (OwnerActor :type "Actor Object Reference") (DeltaSeconds :type "Float (single-precision)"))
  (bind _returnvalue (`KismetMathLibrary.FClamp` (* (`self.Time`) 2.0)))
  (set `self.Time` (+ (`self.Time`) DeltaSeconds))
  (`Actor.K2_SetActorRotation` (stale `self.ReceiveExecute` _asbp_npc) (`KismetMathLibrary.RLerp` (`self.OldRotation`) (`KismetMathLibrary.MakeRotator` 0.0 0.0 (`/Game/Blueprints/AI/BP_NPC.LookAtRotation` (stale `self.ReceiveExecute` _asbp_npc))) _returnvalue true) false)
  (if (== _returnvalue 1.0)
    (`self.FinishExecute` true)
    (set `self.Time` 0.0)))