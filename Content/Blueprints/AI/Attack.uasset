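; Behavior tree task that makes a BP_NPC perform a melee-range attack on its Target.
; On execute, an NPC within range calls TryBlock and waits briefly if the target's Aim is positive, then taps its weapon's LMB input and finishes after a delay.
; Tick turns the NPC's yaw toward the target.
; The task fails only for an invalid target; out-of-range, missing-weapon and failed-cast cases still report success.
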(event `self.ReceiveExecute`
  (params (OwnerActor :type "Actor Object Reference"))
  (bind _asaicontroller (cast `AIController` OwnerActor)
    (:`then`
      (bind _asbp_npc (cast `/Game/Blueprints/BP_NPC` (`Controller.K2_GetPawn` _asaicontroller))
        (:`then`
          (bind _target (`/Game/Blueprints/BP_NPC.Target` _asbp_npc))
          (`/Engine/EditorBlueprintResources/StandardMacros.IsValid` _target
            (:`Is Valid`
              (if (< (`KismetMathLibrary.Vector_Distance` (`Actor.K2_GetActorLocation` _target) (`Actor.K2_GetActorLocation` _asbp_npc)) 150.0)
                (if (> (`/Game/MultiplayerFPSEngine/Blueprints/BP_PlayerBase.aim` (`/Game/Blueprints/BP_NPC.Target` _asbp_npc)) 0.0)
                  (`/Game/MultiplayerFPSEngine/Blueprints/BP_PlayerBase.TryBlock` _asbp_npc)
                  (`KismetSystemLibrary.Delay` 0.3))
                (`/Engine/EditorBlueprintResources/StandardMacros.IsValid` (`/Game/MultiplayerFPSEngine/Blueprints/BP_PlayerBase.Weapon_BP` _asbp_npc)
                  (:`Is Valid`
                    (bind _weapon_bp (`/Game/MultiplayerFPSEngine/Blueprints/BP_PlayerBase.Weapon_BP` _asbp_npc))
                    (`/Game/MultiplayerFPSEngine/Blueprints/Weapon/BP_Weapon.LMBPressed` _weapon_bp)
                    (`/Game/MultiplayerFPSEngine/Blueprints/Weapon/BP_Weapon.LMBReleased` _weapon_bp)
                    (`KismetSystemLibrary.Delay` 0.7)
                    (`self.FinishExecute` true))
                  (:`Is Not Valid`
                    (`self.FinishExecute` true)))
                (else
                  (`self.FinishExecute` true))))
            (:`Is Not Valid`
              (`self.FinishExecute` false))))
        (:`CastFailed`
          (`self.FinishExecute` true :!label _label))))
    (:`CastFailed`
      (goto _label))))

(event `self.ReceiveTick`
  (params (OwnerActor :type "Actor Object Reference") (DeltaSeconds :type "Float (single-precision)"))
  (bind _asaicontroller (cast `AIController` OwnerActor))
  (bind _asbp_npc (cast `/Game/Blueprints/BP_NPC` (`Controller.K2_GetPawn` _asaicontroller)))
  (bind (_returnvalue_roll _returnvalue_pitch _returnvalue_yaw) (`KismetMathLibrary.BreakRotator` (`KismetMathLibrary.FindLookAtRotation` (`Actor.K2_GetActorLocation` _asbp_npc) (`Actor.K2_GetActorLocation` (`/Game/Blueprints/BP_NPC.Target` _asbp_npc)))))
  (`Actor.K2_SetActorRotation` _asbp_npc (`KismetMathLibrary.MakeRotator` 0.0 0.0 _returnvalue_yaw) false))