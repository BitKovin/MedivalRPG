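; BP_NPC is an AI-controlled NPC that runs a test behavior tree and can attack with a weapon.
; BeginPlay sets up the blackboard with the player character and starts the tree, while Tick writes the player's location to it every frame.
; The Attack event simulates a left-mouse press and immediate release on its weapon Blueprint.
; Pawn sensing does nothing, as the sight-flag and direct move-to logic are disconnected.
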(event `self.ReceiveBeginPlay`
  (`parent.ReceiveBeginPlay`)
  (bind _asaicontroller (cast `AIController` (`self.GetController`)))
  (bind _blackboardcomponent (`AIController.UseBlackboard` _asaicontroller "/Game/Blueprints/AI/NewBlackboardData.NewBlackboardData"))
  (`BlackboardComponent.SetValueAsObject` _blackboardcomponent "Player" (`GameplayStatics.GetPlayerCharacter` 0))
  (`AIController.RunBehaviorTree` _asaicontroller "/Game/Blueprints/AI/TestBehaviorTree.TestBehaviorTree"))

(event `Attack`
  (bind _weapon_bp (`self.Weapon_BP`))
  (`/Game/MultiplayerFPSEngine/Blueprints/Weapon/BP_Weapon.LMBPressed` _weapon_bp)
  (`/Game/MultiplayerFPSEngine/Blueprints/Weapon/BP_Weapon.LMBReleased` _weapon_bp))

(event `self.PawnSensing.OnSeePawn`
  (params (Pawn :type "Pawn Object Reference")))

(event `self.ReceiveTick`
  (params (DeltaSeconds :type "Float (single-precision)"))
  (`parent.ReceiveTick` DeltaSeconds)
  (`BlackboardComponent.SetValueAsVector` (stale `self.ReceiveBeginPlay` _blackboardcomponent) "VectorKey" (`self.K2_GetActorLocation` (`GameplayStatics.GetPlayerCharacter` 0))))

(fn `UserConstructionScript`
  (`parent.UserConstructionScript`))