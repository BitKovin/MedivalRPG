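; Candle actor that lights up at night, following the level's day-night cycle.
; On BeginPlay it finds and caches the DayNightCycle actor.
; Every Tick it wraps that actor's Time to 24 hours and shows its point light and particle system only between evening and early morning, polling rather than reacting to events.
; It also prints the night-time boolean each frame as debug output.
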(event `self.ReceiveBeginPlay`
  (bind _returnvalue (`GameplayStatics.GetActorOfClass` "/Game/Blueprints/DayNight/DayNightCycle.DayNightCycle_C"))
  (set `self.daynight` _returnvalue))

(event `self.ReceiveTick`
  (params (DeltaSeconds :type "Float (single-precision)"))
  (bind _returnvalue (mod (`/Game/Blueprints/DayNight/DayNightCycle.Time` (`self.daynight`)) 24.0))
  (bind _returnvalue_2 (or (> _returnvalue 19.0) (< _returnvalue 7.0)))
  (`KismetSystemLibrary.PrintString` (`KismetStringLibrary.Conv_BoolToString` _returnvalue_2))
  (`SceneComponent.SetVisibility` (`self.PointLight`) _returnvalue_2 false)
  (`SceneComponent.SetVisibility` (`self.ParticleSystem`) _returnvalue_2 false))

(fn `UserConstructionScript`)