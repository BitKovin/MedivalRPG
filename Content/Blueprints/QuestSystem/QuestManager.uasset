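; Quest manager that starts quests, tracks them in a Quests array and supports saving and loading them.
; StartQuest spawns an actor of the given quest class, adds it to the array and calls its Start.
; Tick removes empty entries and prints each valid quest's name and first objective as debug text.
; Save and Load copy entries by index between Quests and QuestSave, while ComponentsToSave returns nothing.
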(event `self.ReceiveTick`
  (params (DeltaSeconds :type "Float (single-precision)"))
  (`KismetArrayLibrary.Array_RemoveItem` (`self.Quests`))
  (for _array_element (`self.Quests`)
    (`/Engine/EditorBlueprintResources/StandardMacros.IsValid` _array_element
      (:`Is Valid`
        (`KismetSystemLibrary.PrintString` (`KismetStringLibrary.Concat_StrStr` "================================" (`KismetTextLibrary.Conv_TextToString` (`/Game/Blueprints/QuestSystem/Quest.Name` _array_element)) (`KismetTextLibrary.Conv_TextToString` (`|GetArrayItem` (`/Game/Blueprints/QuestSystem/Quest.objectives` _array_element)))) true true (struct :`G` 0.66 :`B` 1.0 :`A` 1.0) (`GameplayStatics.GetWorldDeltaSeconds`))))))

(event `Save`
  (for (_array_element _array_index) (`self.Quests`)
    (`KismetArrayLibrary.Array_Set` (`self.QuestSave`) _array_index (`|ConvertAsset` _array_element) true)))

(event `Load`
  (for (_array_element _array_index) (`self.QuestSave`)
    (`KismetArrayLibrary.Array_Set` (`self.Quests`) _array_index (`|ConvertAsset` _array_element) true)))

(fn `ComponentsToSave`
  (returns (Components :type "Array of ActorComponent Object Reference"))
  (return))

(fn `Start Quest`
  (params (QuestClass :type "/Game/Blueprints/QuestSystem/Quest Class Reference"))
  (bind _returnvalue (`|SpawnActorFromClass` QuestClass (`KismetMathLibrary.MakeTransform` (0.0 0.0 0.0)) "AlwaysSpawn" "OverrideRootScale" null null))
  (`KismetArrayLibrary.Array_Add` (`self.Quests`) _returnvalue)
  (`/Game/Blueprints/QuestSystem/Quest.Start` _returnvalue))