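; Base world item pickup that adds its item object to the player's InventoryComponent when used.
; BeginPlay fills ItemObject from GetDefaultItemObject, which is empty here.
; Successful pickup calls a soft Destroy that sets a Destroyed flag, disables physics and collision, hides the mesh and moves it below the world.
; Save hooks store ItemObject; on load, delayed steps reapply the destroyed state, restore the item and re-enable physics.
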(event `self.ReceiveBeginPlay`
  (`|ExecutionSequence`
    (:`then_0`
      (bind _itemobject (`self.GetDefaultItemObject`))
      (bind _output_get (set `self.ItemObject` _itemobject))
      (`KismetSystemLibrary.PrintString` (`KismetSystemLibrary.GetDisplayName` _output_get)))))

(event `self.Use`
  (params (player :type "/Game/MultiplayerFPSEngine/Blueprints/BP_PlayerBase Object Reference"))
  (bind _added (`/Game/Inventory/InventoryComponent.TryAddItem` (`/Game/MultiplayerFPSEngine/Blueprints/BP_PlayerBase.InventoryComponent` player) (`self.ItemObject`)))
  (`KismetSystemLibrary.PrintString` (`KismetStringLibrary.Conv_BoolToString` _added))
  (if _added
    (`self.Destroy`)))

(event `EMSActorSaveInterface.ActorLoaded`
  (`KismetSystemLibrary.Delay` 0.2)
  (`PrimitiveComponent.SetSimulatePhysics` (`self.Box`) false)
  (if (`self.Destroyed`)
    (`self.Destroy`))
  (`KismetSystemLibrary.Delay` 0.2)
  (set `self.ItemObject` (`|ConvertAsset` (`self.ItemObjectSave`)))
  (`PrimitiveComponent.SetSimulatePhysics` (`self.Box`) true))

(event `EMSActorSaveInterface.ActorPreSave`
  (set `self.ItemObjectSave` (`|ConvertAsset` (`self.ItemObject`))))

(fn `ComponentsToSave`
  (returns (Components :type "Array of ActorComponent Object Reference"))
  (return))

(fn `Destroy`
  (set `self.Destroyed` true)
  (`PrimitiveComponent.SetSimulatePhysics` (`self.Box`) false)
  (`PrimitiveComponent.SetCollisionEnabled` (`self.Box`) "NoCollision")
  (`SceneComponent.K2_SetWorldLocation` (`self.Box`) (0.0 0.0 -1000.0) false true)
  (`SceneComponent.SetVisibility` (`self.StaticMesh`) false true))

(fn `GetDefaultItemObject`
  (returns (itemObject :type "/Game/Inventory/Bp_ItemObject Object Reference"))
  (return null))

(fn `UserConstructionScript`)