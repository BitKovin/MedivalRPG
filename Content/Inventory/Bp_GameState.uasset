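; Game state Blueprint for the inventory system that provides a function for spawning an item into the world from an actor.
; SpawnItemFromActor spawns the item object's class just in front of the given actor, matching only its yaw and ignoring collisions.
; The new actor receives the item object and its weapon actor reference.
; The GroundClamp input is unused, and the event graph and construction script are empty.
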(fn `SpawnItemFromActor`
  (params (actor :type "Actor Object Reference") (itemObject :type "/Game/Inventory/Bp_ItemObject Object Reference") (GroundClamp :type Boolean))
  (locals (SpawnLocation :type "Vector Structure" :default (0.0 0.0 0.0)))
  (bind (_returnvalue_roll _returnvalue_pitch _returnvalue_yaw) (`KismetMathLibrary.BreakRotator` (`self.K2_GetActorRotation` actor)))
  (`|ExecutionSequence`
    (:`then_0`
      (bind _output_get (set `local.SpawnLocation` (+ (`self.K2_GetActorLocation` actor) (* (`self.GetActorForwardVector` actor) 20.0))))
      (`|SpawnActorFromClass` (`/Game/Inventory/Bp_ItemObject.ItemClass` itemObject) (`KismetMathLibrary.MakeTransform` _output_get (`KismetMathLibrary.MakeRotator` 0.0 0.0 _returnvalue_yaw)) "AlwaysSpawn" "OverrideRootScale" null itemObject (`/Game/Inventory/Bp_ItemObject.weaponActor` itemObject) null))))

(fn `UserConstructionScript`)