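; BP_knife is a world pickup for a knife that can be placed in the player's inventory.
; On Use, it offers its item object to the player's InventoryComponent and destroys itself if the add succeeds.
; GetDefaultItemObject constructs that Bp_ItemObject as a weapon with a rectangular size, normal and rotated icons, the weapon actor, and its own class as the item class.
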(event `/Game/MultiplayerFPSEngine/Blueprints/BP_Useble.Use`
  (params (player :type "/Game/MultiplayerFPSEngine/Blueprints/BP_PlayerBase Object Reference"))
  (bind _itemobject (`self.GetDefaultItemObject`))
  (bind _added (`/Game/Inventory/InventoryComponent.TryAddItem` (`/Game/MultiplayerFPSEngine/Blueprints/BP_PlayerBase.InventoryComponent` player) _itemobject))
  (if _added
    (`self.K2_DestroyActor`)))

(fn `GetDefaultItemObject`
  (returns (itemObject :type "/Game/Inventory/Bp_ItemObject Object Reference"))
  (bind _returnvalue (`|GenericCreateObject` "/Game/Inventory/Bp_ItemObject.Bp_ItemObject_C" self (make `IntPoint` 3 2) "/Game/Inventory/M_Icon_knife.M_Icon_knife" "/Game/Inventory/M_Icon_knife_Rotated.M_Icon_knife_Rotated" "BP_knife_C" (`self.weaponActor`) true))
  (return _returnvalue))

(fn `UserConstructionScript`
  (`parent.UserConstructionScript`))