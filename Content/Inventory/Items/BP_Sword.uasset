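; BP_Sword is a world sword item that moves into the player's grid inventory when used.
; Use passes a new Bp_ItemObject, carrying footprint, icons and weapon flags, to the player's InventoryComponent and destroys the actor if the add succeeds.
; GetDefaultItemObject spawns a W_Sword weapon actor below the origin when WeaponActor is invalid, then links it to the item object.
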(event `/Game/MultiplayerFPSEngine/Blueprints/BP_Useble.Use`
  (params (player :type "/Game/MultiplayerFPSEngine/Blueprints/BP_PlayerBase Object Reference"))
  (bind _itemobject (`self.GetDefaultItemObject`))
  (bind _added (`/Game/Inventory/InventoryComponent.TryAddItem` (`/Game/MultiplayerFPSEngine/Blueprints/BP_PlayerBase.InventoryComponent` player) _itemobject))
  (if _added
    (`self.K2_DestroyActor`)))

(fn `GetDefaultItemObject`
  (returns (itemObject :type "/Game/Inventory/Bp_ItemObject Object Reference"))
  (`/Engine/EditorBlueprintResources/StandardMacros.IsValid` (`|ConvertAsset` (`self.weaponActor`))
    (:`Is Valid`
      _)
    (:`Is Not Valid`
      (bind _returnvalue (`|SpawnActorFromClass` "/Game/MultiplayerFPSEngine/Blueprints/Weapons/Sword/W_Sword.W_Sword_C" (`KismetMathLibrary.MakeTransform` (0.0 0.0 -1000.0)) "Undefined" "OverrideRootScale" null false true false null))
      (set `self.weaponActor` (`|ConvertAsset` _returnvalue))))
  (bind _returnvalue_2 (`|GenericCreateObject` "/Game/Inventory/Bp_ItemObject.Bp_ItemObject_C" self (make `IntPoint` 2 6) "/Game/Inventory/Icons/Sword/M_Icon_Sword.M_Icon_Sword" "/Game/Inventory/Icons/Sword/M_Icon_Sword_Rotated.M_Icon_Sword_Rotated" "BP_Sword_C" (`self.weaponActor`) true true))
  (return _returnvalue_2))

(fn `UserConstructionScript`
  (`parent.UserConstructionScript`))