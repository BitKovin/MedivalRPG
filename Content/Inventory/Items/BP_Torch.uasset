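; BP_Torch is the inventory item Blueprint for a torch, flagged as a weapon.
; Its GetDefaultItemObject builds a Bp_ItemObject with the torch's grid size, normal and rotated icons, item class and in-slot rotation.
; If no valid WeaponActor exists, it first spawns a W_Torch below the world origin and passes that actor to the item object.
; The construction script only calls the parent, and the event graph is unused.
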(fn `GetDefaultItemObject`
  (returns (itemObject :type "/Game/Inventory/Bp_ItemObject Object Reference"))
  (`/Engine/EditorBlueprintResources/StandardMacros.IsValid` (`|ConvertAsset` (`self.weaponActor`))
    (:`Is Valid`
      _)
    (:`Is Not Valid`
      (bind _returnvalue (`|SpawnActorFromClass` "/Game/MultiplayerFPSEngine/Blueprints/Weapons/Sword/W_Torch.W_Torch_C" (`KismetMathLibrary.MakeTransform` (0.0 0.0 -1000.0)) "Undefined" "OverrideRootScale" null false true false null))
      (set `self.weaponActor` (`|ConvertAsset` _returnvalue))))
  (bind _returnvalue_2 (`|GenericCreateObject` "/Game/Inventory/Bp_ItemObject.Bp_ItemObject_C" self (make `IntPoint` 1 4) "/Game/Inventory/Icons/Torch/M_Icon_Torch.M_Icon_Torch" "/Game/Inventory/Icons/Torch/M_Icon_Torch_Rotated.M_Icon_Torch_Rotated" (`GameplayStatics.GetObjectClass` self) (`self.weaponActor`) true true (`|ConvertAsset` self)))
  (return _returnvalue_2))

(fn `UserConstructionScript`
  (`parent.UserConstructionScript`))