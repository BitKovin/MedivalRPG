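; BP_SwordWooden is an inventory item for a wooden sword, supplying the item object that describes it as a weapon.
; GetDefaultItemObject first spawns a W_SwordWooden actor below the world origin if no valid WeaponActor is cached.
; It then constructs a Bp_ItemObject carrying grid size, normal and rotated icons, slot settings, the weapon actor and itself.
; The item object's ItemClass is BP_Sword rather than this wooden variant.
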(fn `GetDefaultItemObject`
  (returns (itemObject :type "/Game/Inventory/Bp_ItemObject Object Reference"))
  (`/Engine/EditorBlueprintResources/StandardMacros.IsValid` (`|ConvertAsset` (`self.weaponActor`))
    (:`Is Valid`
      _)
    (:`Is Not Valid`
      (bind _returnvalue (`|SpawnActorFromClass` "/Game/MultiplayerFPSEngine/Blueprints/Weapons/Sword/W_SwordWooden.W_SwordWooden_C" (`KismetMathLibrary.MakeTransform` (0.0 0.0 -1000.0)) "Undefined" "OverrideRootScale" null false false false null))
      (set `self.weaponActor` (`|ConvertAsset` _returnvalue))))
  (bind _returnvalue_2 (`|GenericCreateObject` "/Game/Inventory/Bp_ItemObject.Bp_ItemObject_C" self (make `IntPoint` 2 6) "/Game/Inventory/Icons/Sword/M_Icon_Sword.M_Icon_Sword" "/Game/Inventory/Icons/Sword/M_Icon_Sword_Rotated.M_Icon_Sword_Rotated" "/Game/Inventory/Items/BP_Sword.BP_Sword_C" (`self.weaponActor`) true true (`|ConvertAsset` self) -1 0 0 0.0 1))
  (return _returnvalue_2))

(fn `UserConstructionScript`
  (`parent.UserConstructionScript`))