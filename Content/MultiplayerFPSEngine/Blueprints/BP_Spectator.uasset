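; Spectator actor that lets the local player watch living teammates through their cameras.
; Tick rebuilds the Team list from all BP_PlayerBase actors on the player's team with health above zero.
; After a zero delay on BeginPlay, and on each left click, it steps backward through that list, wrapping to the last entry.
; UpdateTarget flags only the target as Spectating, then attaches and snaps to its Camera1.
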(event `UpdateTarget`
  (bind _target (`self.target`))
  (bind _camera1 (`/Game/MultiplayerFPSEngine/Blueprints/BP_PlayerBase.Camera1` _target))
  (bind (_returnvalue_location _returnvalue_rotation) (`KismetMathLibrary.BreakTransform` (`SceneComponent.K2_GetComponentToWorld` _camera1)))
  (bind _outactors (`GameplayStatics.GetAllActorsOfClass` "/Game/MultiplayerFPSEngine/Blueprints/BP_PlayerBase.BP_PlayerBase_C"))
  (for _array_element _outactors
    (set `/Game/MultiplayerFPSEngine/Blueprints/BP_PlayerBase.spectating` false _array_element))
  (set `/Game/MultiplayerFPSEngine/Blueprints/BP_PlayerBase.spectating` true _target)
  (`self.K2_AttachToComponent` _camera1 "None" "KeepWorld" "KeepWorld" "KeepWorld")
  (`self.K2_SetActorLocation` _returnvalue_location)
  (`self.K2_SetActorRotation` _returnvalue_rotation))

(event `self.ReceiveBeginPlay`
  (bind _team (`self.team`))
  (bind _returnvalue (`KismetArrayLibrary.Array_LastIndex` _team))
  (`KismetSystemLibrary.Delay` 0.0)
  (if (> (`KismetArrayLibrary.Array_Length` (`self.team`)) 0) :!label _label
    (`/Engine/EditorBlueprintResources/StandardMacros.IsValid` (`|GetArrayItem` _team (- (`self.curentPlayerIndex`) 1))
      (:`Is Valid`
        (set `self.curentPlayerIndex` (- (`self.curentPlayerIndex`) 1))
        (set `self.target` (`|GetArrayItem` _team (`self.curentPlayerIndex`)))
        (`self.UpdateTarget`))
      (:`Is Not Valid`
        (set `self.curentPlayerIndex` _returnvalue)
        (set `self.target` (`|GetArrayItem` _team _returnvalue))
        (`self.UpdateTarget`)))))

(event `Key|LeftMouseButton`
  (params (Key :type "Key Structure"))
  (:`Pressed`
    (goto _label)))

(event `Key|RightMouseButton`
  (params (Key :type "Key Structure")))

(event `self.ReceiveTick`
  (params (DeltaSeconds :type "Float (single-precision)"))
  (`KismetArrayLibrary.Array_Clear` (`self.team`))
  (bind _outactors (`GameplayStatics.GetAllActorsOfClass` "/Game/MultiplayerFPSEngine/Blueprints/BP_PlayerBase.BP_PlayerBase_C"))
  (for _array_element _outactors
    (if (and (== (`/Game/MultiplayerFPSEngine/Blueprints/BP_PlayerBase.team` _array_element) (`/Game/MultiplayerFPSEngine/Animations/Blueprints/PlayerState.Team` (cast `/Game/MultiplayerFPSEngine/Animations/Blueprints/PlayerState` (`Controller.PlayerState` (`GameplayStatics.GetPlayerController` 0)) :!pure true))) (> (`/Game/MultiplayerFPSEngine/Blueprints/BP_PlayerBase.health` _array_element) 0.0))
      (`KismetArrayLibrary.Array_Add` (`self.team`) _array_element))))

(fn `UserConstructionScript`)