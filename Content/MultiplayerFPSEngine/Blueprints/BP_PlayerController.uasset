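; BP_PlayerController is the FPS player controller, handling pause, save/load and match messaging.
; Escape or P toggles the pause menu, stopping aim and pausing the game.
; F6 saves actors asynchronously behind a saving widget, while F7 flags the GameInstance and reopens the level so BeginPlay loads the save.
; Save hooks preserve control rotation and QuestManager state; other events relay kill feed, team wins and ping.
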(event `self.ReceiveBeginPlay`
  (bind _asbp_game_instance (cast `/Game/MultiplayerFPSEngine/Blueprints/BP_GameInstance` (`GameplayStatics.GetGameInstance`)))
  (if (`/Game/MultiplayerFPSEngine/Blueprints/BP_GameInstance.LoadGame` _asbp_game_instance)
    (`EMSAsyncLoadGame.AsyncLoadActors` 3 true)))

(event `Key|Escape` :paused true
  (params (Key :type "Key Structure"))
  (:`Pressed`
    (`/Engine/EditorBlueprintResources/StandardMacros.IsValid` (`self.pauseMenu`) :!label _label
      (:`Is Valid`
        (`/Game/MultiplayerFPSEngine/UI/PauseMenu.Resume` (`self.pauseMenu`)))
      (:`Is Not Valid`
        (bind _returnvalue (`|CreateWidget` "/Game/MultiplayerFPSEngine/UI/PauseMenu.PauseMenu_C"))
        (`UserWidget.AddToViewport` _returnvalue 5)
        (set `self.pauseMenu` _returnvalue)
        (bind _asbp_player_base (cast `/Game/MultiplayerFPSEngine/Blueprints/BP_PlayerBase` (`GameplayStatics.GetPlayerCharacter` 0)))
        (`/Game/MultiplayerFPSEngine/Blueprints/BP_PlayerBase.StopAim` _asbp_player_base)
        (`GameplayStatics.SetGamePaused` true)))))

(event `Key|P` :paused true
  (params (Key :type "Key Structure"))
  (:`Pressed`
    (goto _label)))

(event `PrintKillFeed`
  (params (killer :type String) (killed :type String) (weapon :type String) (hs :type Boolean))
  (`self.ShowInKillFeed` killer killed weapon hs))

(event `SetPing`
  (params (ping :type Integer))
  (set `self.ping` ping))

(event `self.ReceiveTick`
  (params (DeltaSeconds :type "Float (single-precision)"))
  (`|ExecutionSequence`
    (:`then_1`
      (if (`self.IsLocalController`)
        _))))

(event `TeamWonMsg`
  (params (team :type Byte))
  (`self.TeamWon` team))

(event `Key|F6`
  (params (Key :type "Key Structure"))
  (:`Pressed`
    (`EMSAsyncSaveGame.AsyncSaveActors` 3
      (:`then`
        (bind _returnvalue (`|CreateWidget` "/Game/MultiplayerFPSEngine/UI/SavingGame.SavingGame_C"))
        (`UserWidget.AddToViewport` _returnvalue 0))
      (:`OnCompleted`
        (`Widget.RemoveFromParent` _returnvalue)))))

(event `Key|F7`
  (params (Key :type "Key Structure"))
  (:`Pressed`
    (bind _asbp_game_instance (cast `/Game/MultiplayerFPSEngine/Blueprints/BP_GameInstance` (`GameplayStatics.GetGameInstance`)))
    (set `/Game/MultiplayerFPSEngine/Blueprints/BP_GameInstance.LoadGame` true _asbp_game_instance)
    (bind _returnvalue (`GameplayStatics.GetCurrentLevelName` true))
    (`GameplayStatics.OpenLevel` (`KismetStringLibrary.Conv_StringToName` _returnvalue))))

(event `EMSActorSaveInterface.ActorPreSave`
  (set `self.Rotation` (`self.GetControlRotation`))
  (`/Game/Blueprints/QuestSystem/QuestManager.Save` (`self.QuestManager`)))

(event `EMSActorSaveInterface.ActorLoaded`
  (`self.SetControlRotation` (`self.Rotation`))
  (bind _returnvalue (`|CreateWidget` "/Game/MultiplayerFPSEngine/UI/LoadingEndFade.LoadingEndFade_C"))
  (`UserWidget.AddToViewport` _returnvalue 0)
  (`KismetSystemLibrary.Delay` 5.0)
  (`Widget.RemoveFromParent` _returnvalue)
  (`/Game/Blueprints/QuestSystem/QuestManager.Load` (`self.QuestManager`)))

(fn `ComponentsToSave`
  (returns (Components :type "Array of ActorComponent Object Reference"))
  (return (`|MakeArray` (`self.QuestManager`) :!type "ActorComponent Object Reference")))

(fn `UserConstructionScript`)