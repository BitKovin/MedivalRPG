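; BP_Weapon is the base weapon for a multiplayer FPS, with empty hooks for shooting, input, pickup and bullet hits.
; Each tick it calls Shoot while it has a player, and calls the player's LMBRServer if it is equipped with an empty clip.
; Damage routes through the player, shooting animation state relays from server to client, and the authority destroys the weapon with its player.
; Save/load events preserve the player reference.
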(event `Shoot`)

(event `LMBPressed`)

(event `LMBReleased`)

(event `DamageActor`
  (params (damage :type "Float (double-precision)") (actor :type "Actor Object Reference (by ref)") (hitbox :type String))
  (bind _player (`self.player`))
  (`/Game/MultiplayerFPSEngine/Blueprints/BP_PlayerBase.Damage` _player actor damage hitbox (`Pawn.GetController` _player) self))

(event `SetInClip`
  (params (val :type Integer))
  (set `self.InClip` val))

(event `self.ReceiveBeginPlay`
  (if (`self.preSpawn`)
    (`PrimitiveComponent.SetSimulatePhysics` (`self.Box`) false)))

(event `isShootingServer`
  (params (val :type Boolean :default false))
  (bind _output_get (set `self.shooting_animation` val))
  (`self.isShootingClient` _output_get))

(event `PickUp`)

(event `isShootingClient`
  (params (val :type Boolean :default false))
  (set `self.shooting_animation` val))

(event `self.ReceiveTick`
  (params (DeltaSeconds :type "Float (single-precision)"))
  (bind _player (`self.player`))
  (`|ExecutionSequence`
    (:`then_0`
      (`/Engine/EditorBlueprintResources/StandardMacros.IsValid` _player
        (:`Is Valid`
          (`self.Shoot`)
          (if (== (`/Game/MultiplayerFPSEngine/Blueprints/BP_PlayerBase.Weapon_BP` _player) self)
            (if (<= (`self.InClip`) 0)
              (`/Game/MultiplayerFPSEngine/Blueprints/BP_PlayerBase.LMBRServer` (`self.player`)))))))
    (:`then_1`
      (`/Engine/EditorBlueprintResources/StandardMacros.IsValid` (`self.player`)
        (:`Is Valid`
          (`/Engine/EditorBlueprintResources/StandardMacros.DoOnce` false :!label _label
            (:`Completed`
              (`/Engine/EditorBlueprintResources/ActorMacros.Switch Has Authority`
                (:`Authority`
                  (add `self.OnDestroyed` (`self.player`) (delegate `OnPlayerDestroyed`)))))))
        (:`Is Not Valid`
          (goto _label :!via `Reset`))))))

(event `OnPlayerDestroyed` :!signature `self.OnDestroyed`
  (params (DestroyedActor :type "Actor Object Reference"))
  (`self.K2_DestroyActor`))

(event `EMSActorSaveInterface.ActorPreSave`
  (set `self.playerSave` (`|ConvertAsset` (`self.player`))))

(event `EMSActorSaveInterface.ActorLoaded`
  (`EMSAsyncWait.AsyncWaitForOperation`
    (:`OnCompleted`
      (set `self.player` (`|ConvertAsset` (`self.playerSave`))))))

(fn `BulletHit`
  (params (Location :type "Vector Structure") (Normal :type "Vector Structure") (mat :type "PhysicalMaterial Object Reference")))

(fn `CalculateSpray`
  (returns (spray :type "Float (double-precision)"))
  (return (`self.spread`)))

(fn `ComponentsToSave`
  (returns (Components :type "Array of ActorComponent Object Reference"))
  (return))

(fn `UserConstructionScript`)