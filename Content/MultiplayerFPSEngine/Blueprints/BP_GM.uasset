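; Game mode base for a two-team multiplayer FPS, handling player spawning, spectators and team bookkeeping.
; SpawnPlayer possesses a pawn at its team's start and fills three weapon slots; other events create spectators, drop leavers from teams, broadcast wins and destroy "round"-tagged actors.
; Join, death and round-start events are empty: team balancing, scoring, kill feed, respawn and SortPlayersByScore scoreboard logic sit in unconnected nodes.
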(event `MakeSpectator`
  (params (controller :type "/Game/MultiplayerFPSEngine/Blueprints/BP_PlayerController Object Reference"))
  (bind _returnvalue (`|SpawnActorFromClass` "/Game/MultiplayerFPSEngine/Blueprints/BP_Spectator.BP_Spectator_C" (`KismetMathLibrary.MakeTransform` (0.0 0.0 0.0)) "Undefined" "OverrideRootScale" null null))
  (`Controller.Possess` controller _returnvalue)
  (`SceneComponent.K2_SetRelativeLocationAndRotation` :`self` (`self.DefaultSceneRoot`) :`bTeleport` true))

(event `PlayerDied`
  (params (playerController :type "/Game/MultiplayerFPSEngine/Blueprints/BP_PlayerController Object Reference") (character :type "Character Object Reference")))

(event `self.ReceiveTick`
  (params (DeltaSeconds :type "Float (single-precision)")))

(event `self.K2_PostLogin`
  (params (NewPlayer :type "PlayerController Object Reference")))

(event `OnPlayerJoin`
  (params (`player controller` :type "/Game/MultiplayerFPSEngine/Blueprints/BP_PlayerController Object Reference")))

(event `RoundStart`)

(event `TeamWonMsg`
  (params (team :type Byte))
  (bind _outactors (`GameplayStatics.GetAllActorsOfClass` "/Game/MultiplayerFPSEngine/Blueprints/BP_PlayerController.BP_PlayerController_C"))
  (for _array_element _outactors
    (`/Game/MultiplayerFPSEngine/Blueprints/BP_PlayerController.TeamWonMsg` _array_element team)))

(event `self.ReceiveBeginPlay`)

(event `self.K2_OnLogout`
  (params (ExitingController :type "Controller Object Reference"))
  (bind _asbp_player_controller (cast `/Game/MultiplayerFPSEngine/Blueprints/BP_PlayerController` ExitingController))
  (bind _asplayer_state (cast `/Game/MultiplayerFPSEngine/Animations/Blueprints/PlayerState` (`Controller.PlayerState` _asbp_player_controller)))
  (`KismetArrayLibrary.Array_RemoveItem` (select `byte` (`/Game/MultiplayerFPSEngine/Animations/Blueprints/PlayerState.Team` _asplayer_state) :`0` (`self.TeamA`) :`1` (`self.TeamB`)) _asbp_player_controller))

(event `ClearLevel`
  (bind _outactors (`GameplayStatics.GetAllActorsOfClassWithTag` "/Script/Engine.Actor" "round"))
  (for _array_element _outactors
    (`self.K2_DestroyActor` _array_element)))

(event `SpawnPlayer`
  (params (controller :type "/Game/MultiplayerFPSEngine/Blueprints/BP_PlayerController Object Reference"))
  (bind _team (`/Game/MultiplayerFPSEngine/Animations/Blueprints/PlayerState.Team` (cast `/Game/MultiplayerFPSEngine/Animations/Blueprints/PlayerState` (`Controller.PlayerState` controller) :!pure true)))
  (bind (_returnvalue_location _returnvalue_rotation) (`KismetMathLibrary.BreakTransform` (`self.GetTransform` (`self.K2_FindPlayerStart` controller (select `byte` _team :`0` "A" :`1` "B")))))
  (bind _returnvalue (`|SpawnActorFromClass` "/Game/MultiplayerFPSEngine/Blueprints/BP_PlayerBase.BP_PlayerBase_C" (`KismetMathLibrary.MakeTransform` _returnvalue_location (struct :`Yaw` 35.0)) "Undefined" "OverrideRootScale" null null))
  (set `/Game/MultiplayerFPSEngine/Blueprints/BP_PlayerBase.team` _team _returnvalue)
  (`Controller.Possess` controller _returnvalue)
  (`/Game/MultiplayerFPSEngine/Blueprints/BP_PlayerBase.SetRotation` _returnvalue _returnvalue_rotation)
  (bind _returnvalue_2 (`|SpawnActorFromClass` "/Game/MultiplayerFPSEngine/Blueprints/Weapons/AK/BP_KA.BP_KA_C" (`KismetMathLibrary.MakeTransform` (0.0 0.0 0.0)) "Undefined" "OverrideRootScale" null true true true null))
  (bind _slots (`/Game/MultiplayerFPSEngine/Blueprints/BP_PlayerBase.Slots` _returnvalue))
  (`KismetArrayLibrary.Array_Set` _slots 0 _returnvalue_2 true)
  (bind _returnvalue_3 (`|SpawnActorFromClass` "/Game/MultiplayerFPSEngine/Blueprints/Weapons/ShotGun/Shotgun.Shotgun_C" (`KismetMathLibrary.MakeTransform` (0.0 0.0 0.0)) "Undefined" "OverrideRootScale" null false true false null))
  (`KismetArrayLibrary.Array_Set` _slots 1 _returnvalue_3 true)
  (bind _returnvalue_4 (`|SpawnActorFromClass` "/Game/MultiplayerFPSEngine/Blueprints/Weapons/AK/BP_KA.BP_KA_C" (`KismetMathLibrary.MakeTransform` (0.0 0.0 0.0)) "Undefined" "OverrideRootScale" null true true true null))
  (`KismetArrayLibrary.Array_Set` _slots 2 _returnvalue_4 true))

(fn `SortPlayersByScore`
  (params (NewParam1 :type "Array of /Game/MultiplayerFPSEngine/Blueprints/BP_PlayerController Object Reference"))
  (returns (NewParam :type "Array of /Game/MultiplayerFPSEngine/Blueprints/BP_PlayerScore Structure"))
  (locals (LocalCache :type "Array of /Game/MultiplayerFPSEngine/Blueprints/BP_PlayerController Object Reference") (Out :type "Array of /Game/MultiplayerFPSEngine/Blueprints/BP_PlayerScore Structure"))
  (bind _returnvalue (`KismetArrayLibrary.Array_Length` NewParam1))
  (bind _playerstate (`Controller.PlayerState` (`|GetArrayItem` NewParam1)))
  (bind _asplayer_state (cast `/Game/MultiplayerFPSEngine/Animations/Blueprints/PlayerState` _playerstate :!pure true))
  (`|ExecutionSequence`
    (:`then_0`
      (if (> _returnvalue 1)
        (for _array_element _
          (for (_array_element_2 _array_index) (`local.LocalCache`)
            (if (> (`/Game/MultiplayerFPSEngine/Animations/Blueprints/PlayerState.PlayerScore` (cast `/Game/MultiplayerFPSEngine/Animations/Blueprints/PlayerState` (`Controller.PlayerState` _array_element) :!pure true)) (`/Game/MultiplayerFPSEngine/Animations/Blueprints/PlayerState.PlayerScore` (cast `/Game/MultiplayerFPSEngine/Animations/Blueprints/PlayerState` (`Controller.PlayerState` _array_element_2) :!pure true)))
              (`KismetArrayLibrary.Array_Insert` (`local.LocalCache`) _array_element _array_index)
              (break)))
          (`KismetArrayLibrary.Array_Add` (`local.LocalCache`) _array_element))
        (for _array_element_3 (`local.LocalCache`)
          (bind _asplayer_state_2 (cast `/Game/MultiplayerFPSEngine/Animations/Blueprints/PlayerState` (`Controller.PlayerState` _array_element_3) :!pure true))
          (`KismetArrayLibrary.Array_Add` (`local.Out`) (make `/Game/MultiplayerFPSEngine/Blueprints/BP_PlayerScore` (`PlayerState.GetPlayerName` (`Controller.PlayerState` _array_element_3)) (`/Game/MultiplayerFPSEngine/Animations/Blueprints/PlayerState.PlayerScore` _asplayer_state_2) (`/Game/MultiplayerFPSEngine/Animations/Blueprints/PlayerState.kills` _asplayer_state_2) (`/Game/MultiplayerFPSEngine/Animations/Blueprints/PlayerState.death` _asplayer_state_2) (`/Game/MultiplayerFPSEngine/Animations/Blueprints/PlayerState.level` _asplayer_state_2) (`KismetMathLibrary.Conv_ByteToInt` (`PlayerState.Ping` _asplayer_state_2)))))
        (elif (> _returnvalue 0)
          (return (`|MakeArray` (make `/Game/MultiplayerFPSEngine/Blueprints/BP_PlayerScore` (`PlayerState.GetPlayerName` _playerstate) (`/Game/MultiplayerFPSEngine/Animations/Blueprints/PlayerState.PlayerScore` _asplayer_state) (`/Game/MultiplayerFPSEngine/Animations/Blueprints/PlayerState.kills` _asplayer_state) (`/Game/MultiplayerFPSEngine/Animations/Blueprints/PlayerState.death` _asplayer_state) (`/Game/MultiplayerFPSEngine/Animations/Blueprints/PlayerState.level` _asplayer_state) (`KismetMathLibrary.Conv_ByteToInt` (`PlayerState.Ping` _asplayer_state))) :!type "/Game/MultiplayerFPSEngine/Blueprints/BP_PlayerScore Structure")))))
    (:`then_1`
      (return (`local.Out`)))))

(fn `UserConstructionScript`)