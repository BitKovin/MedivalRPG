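; AK rifle weapon Blueprint for a multiplayer FPS, with optional sight and vertical grip.
; Gates allow firing after the pickup draw delay while the trigger is held, provided the player has ammo and isn't reloading or running.
; The local player line-traces from the camera, applies recoil and passes damage to Player; others only play positional audio.
; A timeline grows spread per shot, Tick recovers it after a pause, and aiming removes it.
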(event `SprayReset`
  (`/Engine/EditorBlueprintResources/StandardMacros.Gate` true :!label _label
    (:`Exit`
      (bind _output_get (set `self.spread` (`KismetMathLibrary.FClamp` (- (stale _output_get) (* (`GameplayStatics.GetWorldDeltaSeconds`) 100.0)) 0.0 60.0))))))

(event `self.PickUp`
  (bind _returnvalue (/ 0.1 -5.0))
  (bind _returnvalue_2 (/ 0.8 -5.0))
  (bind _player (`self.player`))
  (bind _player_2 (`self.player`))
  (bind _shell (`self.shell`))
  (bind _startspray (`self.startSpray`))
  (bind _player_3 (`self.player`))
  (bind _camera1 (`/Game/MultiplayerFPSEngine/Blueprints/BP_PlayerBase.Camera1` (`self.player`)))
  (set `self.drawing` true)
  (`|ExecutionSequence`
    (:`then_0`
      (`KismetSystemLibrary.Delay` 0.1)
      (set `self.drawing` false)
      (`KismetSystemLibrary.Delay` 0.4)
      (goto _label_2 :!via `Open`))
    (:`then_1`
      (goto _label_2 :!via `Close`))))

(event `self.Shoot`
  (bind _returnvalue (/ 0.1 -5.0))
  (bind _returnvalue_2 (/ 0.8 -5.0))
  (bind _player (`self.player`))
  (bind _player_2 (`self.player`))
  (bind _shell (`self.shell`))
  (bind _startspray (`self.startSpray`))
  (bind _player_3 (`self.player`))
  (bind _camera1 (`/Game/MultiplayerFPSEngine/Blueprints/BP_PlayerBase.Camera1` (`self.player`)))
  ;[1 1 1] can I shoot?
  (`/Engine/EditorBlueprintResources/StandardMacros.Gate` true :!label _label_2
    (:`Exit`
      (`/Engine/EditorBlueprintResources/StandardMacros.Gate` true :!label _label_3
        (:`Exit`
          (`/Engine/EditorBlueprintResources/StandardMacros.IsValid` (`self.player`)
            (:`Is Valid`
              (if (and (`KismetMathLibrary.Conv_IntToBool` (`self.InClip`)) (not (`/Game/MultiplayerFPSEngine/Blueprints/BP_PlayerBase.reloading` _player)) (== (`/Game/MultiplayerFPSEngine/Blueprints/BP_PlayerBase.runProgres` _player) 0.0))
                (set `self.shooting_animation` true)
                (`KismetSystemLibrary.Delay` (`self.shootDelay`))
                (if (`Pawn.IsLocallyControlled` (`self.player`))
                  (`GameplayStatics.PlaySound2D` "/Game/MultiplayerFPSEngine/Sounds/Rifle_Fire_Cue.Rifle_Fire_Cue" 0.5 0.9 0.0 null null false)
                  (if (> (`/Game/MultiplayerFPSEngine/Blueprints/BP_PlayerBase.aim` (`self.player`)) 0.7)
                    (`PlayerController.ClientStartCameraShake` :`self` (`GameplayStatics.GetPlayerController` 0) :`Shake` "/Game/MultiplayerFPSEngine/Blueprints/Weapons/AK/WeaponCameraShake.WeaponCameraShake_C" :`Scale` 0.7)
                    ;[1 1 1] reloil
                    (`Pawn.AddControllerPitchInput` _player_3 (`KismetMathLibrary.SelectFloat` -0.2 -0.25 (`self.Vertgrip`)))
                    (`Pawn.AddControllerYawInput` _player_3 (`KismetMathLibrary.RandomFloatInRange` (* _returnvalue_2 -1.0) _returnvalue_2))
                    (else
                      (`PlayerController.ClientStartCameraShake` :`self` (`GameplayStatics.GetPlayerController` 0) :`Shake` "/Game/MultiplayerFPSEngine/Blueprints/Weapons/AK/WeaponCameraShake.WeaponCameraShake_C" :`Scale` 0.9)
                      (`Pawn.AddControllerPitchInput` _player_2 (`KismetMathLibrary.SelectFloat` -0.1 -0.2 (`self.Vertgrip`)))
                      (`Pawn.AddControllerYawInput` _player_2 (`KismetMathLibrary.RandomFloatInRange` (* _returnvalue -1.0) _returnvalue))))
                  (bind _outhit (`KismetSystemLibrary.LineTraceSingle` (`SceneComponent.K2_GetComponentLocation` _camera1) (+ (`SceneComponent.K2_GetComponentLocation` _camera1) (* (`SceneComponent.GetForwardVector` _camera1) 100000.0) (* (* (`KismetMathLibrary.GreaterGreater_VectorRotator` (`self.randomVector` (`self.CalculateSpray`)) (`SceneComponent.K2_GetComponentRotation` _camera1)) 100.0) (`KismetMathLibrary.Conv_BoolToDouble` (not (> (`/Game/MultiplayerFPSEngine/Blueprints/BP_PlayerBase.aim` (`self.player`)) 0.2))))) "TraceTypeQuery1" false (`|MakeArray` (`self.player`) :!type "Actor Object Reference") "None" true (struct :`G` 0.076852 :`B` 1.0 :`A` 1.0)))
                  (bind _output_get (set `self.InClip` (- (stale _output_get) 1)))
                  ;[1 1 1] hit
                  (`|ExecutionSequence`
                    (:`then_0`
                      (set `self.startSpray` (`self.spread`))
                      (`|ExecutionSequence`
                        (:`then_0`
                          (`|ExecutionSequence`
                            (:`then_0`
                              (`KismetSystemLibrary.RetriggerableDelay` 0.2)
                              (goto _label :!via `Open`))
                            (:`then_1`
                              (goto _label :!via `Close`))))
                        (:`then_1`
                          (bind (_direction _newtrack_0) (`Timeline|SmoothSpray` :!via `PlayFromStart`)
                            (:`Update`
                              (set `self.spread` (`KismetMathLibrary.FClamp` (`KismetMathLibrary.Lerp` _startspray (+ _startspray (`KismetMathLibrary.SelectFloat` 4.0 3.0 (`self.Vertgrip`))) _newtrack_0) 0.0 (`KismetMathLibrary.SelectFloat` 40.0 20.0 (`self.Vertgrip`)))))))))
                    (:`then_1`
                      (`/Game/MultiplayerFPSEngine/Blueprints/BP_PlayerBase.Damage` (`self.player`) (`.HitActor` (`GameplayStatics.BreakHitResult` _outhit)) (`self.damage`) (`KismetStringLibrary.Conv_NameToString` (`.HitBoneName` (`GameplayStatics.BreakHitResult` _outhit))) null self)
                      (bind _returnvalue_3 (`|SpawnActorFromClass` "/Game/MultiplayerFPSEngine/Blueprints/Weapon/BP_Shell.BP_Shell_C" (`SceneComponent.K2_GetComponentToWorld` _shell) "Undefined" "OverrideRootScale" null null))
                      (`PrimitiveComponent.AddImpulse` (`/Game/MultiplayerFPSEngine/Blueprints/Weapon/BP_Shell.Shell` _returnvalue_3) (+ (* (`SceneComponent.GetForwardVector` _shell) 130.0) (* (`self.GetVelocity` (`self.player`)) 0.5)) "None" false)
                      (`GameplayStatics.SpawnEmitterAttached` null (`self.Muzzle`) "None" (0.0 0.0 0.0) (struct) (1.0 1.0 1.0) "SnapToTargetIncludingScale" true "AutoRelease"))
                    (:`then_2`
                      (if (`GameplayStatics.BreakHitResult` _outhit)
                        (`/Game/MultiplayerFPSEngine/Blueprints/BP_PlayerBase.Hit` (`self.player`) (`.Location` (`GameplayStatics.BreakHitResult` _outhit)) (`.Normal` (`GameplayStatics.BreakHitResult` _outhit)) (`.PhysMat` (`GameplayStatics.BreakHitResult` _outhit))))))
                  (else
                    (`GameplayStatics.PlaySoundAtLocation` "/Game/MultiplayerFPSEngine/Sounds/Rifle_Fire_Cue.Rifle_Fire_Cue" (`self.K2_GetActorLocation`) (struct) 0.8 1.0 0.0 "/Game/MultiplayerFPSEngine/Sounds/ShotSoundAttenuation_.ShotSoundAttenuation_" null self)))
                (else
                  (set `self.shooting_animation` false))))))))))

(event `self.LMBPressed`
  ;[1 1 1] can I shoot?
  (goto _label_3 :!via `Open`))

(event `self.LMBReleased`
  ;[1 1 1] can I shoot?
  (`|ExecutionSequence`
    (:`then_0`
      (goto _label_3 :!via `Close`))
    (:`then_1`
      (set `self.shooting_animation` false))))

(event `self.ReceiveBeginPlay`
  (`parent.ReceiveBeginPlay`))

(event `self.ReceiveTick`
  (params (DeltaSeconds :type "Float (single-precision)"))
  (bind _weapon (`self.Weapon`))
  (`parent.ReceiveTick` DeltaSeconds)
  (`self.SprayReset`)
  (if (`KismetSystemLibrary.IsValid` (`self.player`))
    (`PrimitiveComponent.SetCastShadow` _weapon (not (`Pawn.IsLocallyControlled` (`self.player`))))
    (`PrimitiveComponent.SetCastShadow` (`self.SM_T4_Sight`) (not (`Pawn.IsLocallyControlled` (`self.player`))))
    (`PrimitiveComponent.SetCastShadow` (`self.SM_Vertgrip`) (not (`Pawn.IsLocallyControlled` (`self.player`))))
    (`PrimitiveComponent.SetCastShadow` (`self.Cylinder`) (not (`Pawn.IsLocallyControlled` (`self.player`))))
    (else
      (`PrimitiveComponent.SetCastShadow` _weapon true)
      (`PrimitiveComponent.SetCastShadow` (`self.SM_T4_Sight`) true)
      (`PrimitiveComponent.SetCastShadow` (`self.SM_Vertgrip`) true)
      (`PrimitiveComponent.SetCastShadow` (`self.Cylinder`) true))))

(fn `CalculateSpray`
  (returns (spray :type "Float (double-precision)"))
  (bind _player (`self.player`))
  (`/Engine/EditorBlueprintResources/StandardMacros.IsValid` _player
    (:`Is Valid`
      (return (+ (`self.spread`) (* (`KismetMathLibrary.VSize` (`self.GetVelocity` _player)) 0.01) (`KismetMathLibrary.SelectFloat` 2.0 4.0 (`NavMovementComponent.IsCrouching` (`Character.CharacterMovement` _player))))))))

(fn `UserConstructionScript`
  (`parent.UserConstructionScript`)
  (if (`self.sight`)
    (set `self.AimCameraLocation` (-8.2 12.81 -12.81))
    (else
      (set `self.AimCameraLocation` (-10.5 12.7 -12.77))))
  (`SceneComponent.SetVisibility` (`self.SM_T4_Sight`) (`self.sight`) true))