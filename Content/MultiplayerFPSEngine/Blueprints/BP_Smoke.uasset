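; BP_Smoke is a short-lived smoke volume actor that grows a sphere and obscures the player's view near it.
; A timeline drives a Radius value that scales the sphere on BeginPlay, then the actor destroys itself after a short delay.
; Each tick sets a post-process blend weight from the local camera's distance to the sphere, multiplied by Radius, so the effect strengthens as the camera moves inside.
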(event `self.ReceiveBeginPlay`
  (bind (_direction _radius) (`Timeline|Smoke` :!via `PlayFromStart`)
    (:`Update`
      (`SceneComponent.SetWorldScale3D` (`self.Sphere`) (`KismetMathLibrary.Conv_DoubleToVector` (* _radius 5.0))))
    (:`Finished`
      (`KismetSystemLibrary.Delay` 1.0)
      (`self.K2_DestroyActor`))))

(event `self.ReceiveTick`
  (params (DeltaSeconds :type "Float (single-precision)"))
  (set `PostProcessComponent.BlendWeight` (* (/ (- 320.0 (`KismetMathLibrary.Vector_Distance` (`PlayerCameraManager.GetCameraLocation` (`GameplayStatics.GetPlayerCameraManager` 0)) (`SceneComponent.K2_GetComponentLocation` (`self.Sphere`)))) 70.0) (stale `self.ReceiveBeginPlay` _radius)) (`self.PostProcess`)))

(fn `UserConstructionScript`)