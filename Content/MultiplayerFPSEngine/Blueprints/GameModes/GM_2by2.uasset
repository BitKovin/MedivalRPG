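; Game mode for round-based team elimination, named 2by2, where a team scores by wiping out the other.
; Joining players are balanced between TeamA and TeamB, and play starts once both reach PlayersToStart.
; Deaths award score, broadcast the kill feed, switch victims to spectator and decrement alive counts until a team wins.
; Each round destroys all pawns, then respawns players at team-named starts with a BP_KA and Shotgun.
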(event `CustomEvent_2`
  (params (`player controller` :type "/Game/MultiplayerFPSEngine/Blueprints/BP_PlayerController Object Reference"))
  (bind _asplayer_state (cast `/Game/MultiplayerFPSEngine/Animations/Blueprints/PlayerState` (`Controller.PlayerState` `player controller`) :!pure true))
  (`|ExecutionSequence`
    (:`then_0`
      (`|ExecutionSequence`
        (:`then_0`
          (if (== (`KismetArrayLibrary.Array_Length` (`self.TeamA`)) (`KismetArrayLibrary.Array_Length` (`self.TeamB`)))
            (set `/Game/MultiplayerFPSEngine/Animations/Blueprints/PlayerState.Team` 0 _asplayer_state)
            (else
              (set `/Game/MultiplayerFPSEngine/Animations/Blueprints/PlayerState.Team` (select `bool` (> (`KismetArrayLibrary.Array_Length` (`self.TeamA`)) (`KismetArrayLibrary.Array_Length` (`self.TeamB`))) :`true` 1 :!type "Byte") _asplayer_state))))
        (:`then_1`
          (if (== (`/Game/MultiplayerFPSEngine/Animations/Blueprints/PlayerState.Team` (cast `/Game/MultiplayerFPSEngine/Animations/Blueprints/PlayerState` (`Controller.PlayerState` `player controller`) :!pure true)) 0)
            (`KismetArrayLibrary.Array_Add` (`self.TeamA`) `player controller`)
            (else
              (`KismetArrayLibrary.Array_Add` (`self.TeamB`) `player controller`))))))
    (:`then_1`
      (`KismetSystemLibrary.Delay` 0.0)
      (`self.CheckStart`))))

(event `bWon`
  (bind _output_get (set `self.TeamBScore` (+ (stale _output_get) 1)))
  (`self.TeamWonMsg` 1))

(event `self.K2_OnLogout`
  (params (ExitingController :type "Controller Object Reference"))
  (bind _asbp_player_controller (cast `/Game/MultiplayerFPSEngine/Blueprints/BP_PlayerController` ExitingController))
  (bind _asplayer_state (cast `/Game/MultiplayerFPSEngine/Animations/Blueprints/PlayerState` (`Controller.PlayerState` _asbp_player_controller)))
  (bind _team (`/Game/MultiplayerFPSEngine/Animations/Blueprints/PlayerState.Team` _asplayer_state))
  (`KismetArrayLibrary.Array_RemoveItem` (select `byte` _team :`0` (`self.TeamA`) :`1` (`self.TeamB`)) _asbp_player_controller)
  (if (== _team 0)
    (bind _output_get (set `self.AliveA` (- (stale _output_get) 1)))
    (else
      (bind _output_get_2 (set `self.AliveB` (- (stale _output_get_2) 1))))))

(event `self.K2_PostLogin`
  (params (NewPlayer :type "PlayerController Object Reference")))

(event `aWon`
  (bind _output_get (set `self.TeamAScore` (+ (stale _output_get) 1)))
  (`self.TeamWonMsg` 0))

(event `CustomEvent`
  (params (playerController :type "/Game/MultiplayerFPSEngine/Blueprints/BP_PlayerController Object Reference") (character :type "Character Object Reference"))
  (bind _returnvalue (`PlayerState.GetPlayerName` (`Controller.PlayerState` playerController)))
  (`|ExecutionSequence`
    (:`then_0`
      (bind _asbp_player_base (cast `/Game/MultiplayerFPSEngine/Blueprints/BP_PlayerBase` character))
      (bind _lasthit (`/Game/MultiplayerFPSEngine/Blueprints/BP_PlayerBase.LastHit` _asbp_player_base))
      (`/Engine/EditorBlueprintResources/StandardMacros.IsValid` _lasthit
        (:`Is Valid`
          (bind _asplayer_state (cast `/Game/MultiplayerFPSEngine/Animations/Blueprints/PlayerState` (`Controller.PlayerState` _lasthit)))
          (`/Game/MultiplayerFPSEngine/Animations/Blueprints/PlayerState.AddScore` _asplayer_state 100)
          (if (`/Game/MultiplayerFPSEngine/Blueprints/BP_PlayerBase.LastHeadShot` _asbp_player_base)
            (`/Game/MultiplayerFPSEngine/Animations/Blueprints/PlayerState.AddScore` _asplayer_state 50))
          (`/Game/MultiplayerFPSEngine/Animations/Blueprints/PlayerState.AddKills` _asplayer_state 1)
          (`/Game/MultiplayerFPSEngine/Animations/Blueprints/PlayerState.AddDeath` (cast `/Game/MultiplayerFPSEngine/Animations/Blueprints/PlayerState` (`Controller.PlayerState` (`Pawn.GetController` _asbp_player_base)) :!pure true) 1))))
    (:`then_1`
      (bind _asbp_player_base_2 (cast `/Game/MultiplayerFPSEngine/Blueprints/BP_PlayerBase` character))
      (bind _outactors (`GameplayStatics.GetAllActorsOfClass` "/Game/MultiplayerFPSEngine/Blueprints/BP_PlayerController.BP_PlayerController_C"))
      (for _array_element _outactors
        (bind _lasthitweaponname (`/Game/MultiplayerFPSEngine/Blueprints/BP_PlayerBase.lastHitWeaponName` _asbp_player_base_2))
        (if (not (`KismetStringLibrary.EqualEqual_StrStr` _lasthitweaponname))
          (`/Game/MultiplayerFPSEngine/Blueprints/BP_PlayerController.PrintKillFeed` _array_element (`PlayerState.GetPlayerName` (`Controller.PlayerState` (`/Game/MultiplayerFPSEngine/Blueprints/BP_PlayerBase.LastHit` _asbp_player_base_2))) _returnvalue _lasthitweaponname false)
          (else
            (`/Game/MultiplayerFPSEngine/Blueprints/BP_PlayerController.PrintKillFeed` _array_element "" _returnvalue "Suicide" false)))))
    (:`then_2`
      (`KismetSystemLibrary.Delay` 3.0)
      (`self.MakeSpectator` playerController))
    (:`then_3`
      (if (not (`self.RoundEnd`))
        (bind _asplayer_state_2 (cast `/Game/MultiplayerFPSEngine/Animations/Blueprints/PlayerState` (`Controller.PlayerState` playerController)))
        (if (== (`/Game/MultiplayerFPSEngine/Animations/Blueprints/PlayerState.Team` _asplayer_state_2) 0)
          (set `self.AliveA` (- (`self.AliveA`) 1))
          (else
            (set `self.AliveB` (- (`self.AliveB`) 1))))
        (if (<= (`self.AliveA`) 0)
          (`self.bWon`)
          (set `self.RoundEnd` true :!label _label)
          (`KismetSystemLibrary.Delay` 5.0)
          (`self.RoundStart`)
          (elif (<= (`self.AliveB`) 0)
            (`self.aWon`)
            (goto _label)))))))

(event `self.ReceiveBeginPlay`)

(event `CheckStart`
  (bind _playerstostart (`self.PlayersToStart`))
  (if (and (== (`KismetArrayLibrary.Array_Length` (`self.TeamA`)) _playerstostart) (== (`KismetArrayLibrary.Array_Length` (`self.TeamB`)) _playerstostart))
    (`KismetSystemLibrary.Delay` 1.0)
    (`self.RoundStart`)))

(event `CustomEvent_1`
  (bind _outactors (`GameplayStatics.GetAllActorsOfClass` "/Game/MultiplayerFPSEngine/Blueprints/BP_PlayerBase.BP_PlayerBase_C"))
  (for _array_element _outactors
    (`self.K2_DestroyActor` _array_element))
  (`KismetSystemLibrary.Delay` 0.1)
  (bind _outactors_2 (`GameplayStatics.GetAllActorsOfClass` "/Game/MultiplayerFPSEngine/Blueprints/BP_PlayerController.BP_PlayerController_C"))
  (for _array_element_2 _outactors_2
    (`self.SpawnPlayer` _array_element_2))
  (set `self.warmUp` false)
  (set `self.RoundEnd` false)
  (set `self.AliveA` (`KismetArrayLibrary.Array_Length` (`self.TeamA`)))
  (set `self.AliveB` (`KismetArrayLibrary.Array_Length` (`self.TeamB`))))

(event `CustomEvent_3`
  (params (controller :type "/Game/MultiplayerFPSEngine/Blueprints/BP_PlayerController Object Reference"))
  (bind _returnvalue (`KismetMathLibrary.RandomBool`))
  (bind _team (`/Game/MultiplayerFPSEngine/Animations/Blueprints/PlayerState.Team` (cast `/Game/MultiplayerFPSEngine/Animations/Blueprints/PlayerState` (`Controller.PlayerState` controller) :!pure true)))
  (bind (_returnvalue_location _returnvalue_rotation) (`KismetMathLibrary.BreakTransform` (`self.GetTransform` (`self.K2_FindPlayerStart` controller (select `byte` _team :`0` "A" :`1` "B")))))
  (bind _returnvalue_2 (`|SpawnActorFromClass` "/Game/MultiplayerFPSEngine/Blueprints/BP_PlayerBase.BP_PlayerBase_C" (`KismetMathLibrary.MakeTransform` _returnvalue_location (struct :`Yaw` 35.0)) "Undefined" "OverrideRootScale" null (`GameplayStatics.GetPlayerPawn` 0)))
  (set `/Game/MultiplayerFPSEngine/Blueprints/BP_PlayerBase.team` _team _returnvalue_2)
  (`Controller.Possess` controller _returnvalue_2)
  (bind _returnvalue_3 (`|SpawnActorFromClass` "/Game/MultiplayerFPSEngine/Blueprints/Weapons/AK/BP_KA.BP_KA_C" (`KismetMathLibrary.MakeTransform` (0.0 0.0 -10000.0)) "Undefined" "OverrideRootScale" null _returnvalue true _returnvalue null))
  (bind _slots (`/Game/MultiplayerFPSEngine/Blueprints/BP_PlayerBase.Slots` _returnvalue_2))
  (`KismetArrayLibrary.Array_Set` _slots 0 _returnvalue_3 true)
  (bind _returnvalue_4 (`|SpawnActorFromClass` "/Game/MultiplayerFPSEngine/Blueprints/Weapons/ShotGun/Shotgun.Shotgun_C" (`KismetMathLibrary.MakeTransform` (0.0 0.0 -10000.0)) "Undefined" "OverrideRootScale" null false true false null))
  (`KismetArrayLibrary.Array_Set` _slots 1 _returnvalue_4 true))

(fn `UserConstructionScript`
  (`parent.UserConstructionScript`))