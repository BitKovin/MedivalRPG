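; BP_target is a shootable target that displays the damage it takes on a text render.
; On damage it adds to a running total, updates the text, and calls HitedServer on the instigator's BP_PlayerBase pawn as a non-headshot, non-kill hit.
; A one-second retriggerable delay then zeroes the total without refreshing the text, when that player cast succeeds.
; A timeline that would roll the target when hit is disconnected and never runs.
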(event `RotateClient`
  (params (dmg :type "Float (double-precision)"))
  (bind _output_get (set `self.dmg` (+ (`self.dmg`) dmg)))
  (`TextRenderComponent.K2_SetText` (`self.TextRender`) (`KismetTextLibrary.Conv_DoubleToText` _output_get "HalfToEven")))

(event `self.ReceiveAnyDamage`
  (params (Damage :type "Float (single-precision)") (DamageType :type "DamageType Object Reference") (InstigatedBy :type "Controller Object Reference") (DamageCauser :type "Actor Object Reference"))
  (set `self.hited` true)
  (`self.RotateClient` Damage)
  (bind _asbp_player_base (cast `/Game/MultiplayerFPSEngine/Blueprints/BP_PlayerBase` (`Controller.K2_GetPawn` InstigatedBy)))
  (`/Game/MultiplayerFPSEngine/Blueprints/BP_PlayerBase.HitedServer` _asbp_player_base false false)
  (`KismetSystemLibrary.RetriggerableDelay` 1.0)
  (set `self.dmg` 0.0))

(event `self.ReceiveTick`
  (params (DeltaSeconds :type "Float (single-precision)")))

(fn `UserConstructionScript`
  (`parent.UserConstructionScript`))