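; BP_Sword is a melee weapon that the player swings with the left mouse button.
; A press while not aiming, gated by a Tick-driven cooldown, plays alternating left and right attack montages with a delayed sound and then a short forward capsule trace from the camera.
; The trace result is unused, so no damage is applied here.
; It also clears Drawing on pickup and returns a fixed spray value.
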(event `self.PickUp`
  (set `self.drawing` false))

(event `self.LMBPressed`
  (bind _camera1 (`/Game/MultiplayerFPSEngine/Blueprints/BP_PlayerBase.Camera1` (`self.player`)))
  (bind _returnvalue (`SceneComponent.K2_GetComponentLocation` _camera1))
  (if (and (< (`self.AttackDelay`) 0.0) (< (`/Game/MultiplayerFPSEngine/Blueprints/BP_PlayerBase.aim` (`self.player`)) 0.1))
    (`Character.PlayAnimMontage` (`self.player`) (select `bool` (`self.attack`) :`false` "/Game/MultiplayerFPSEngine/Sword/AttackLeft_Montage.AttackLeft_Montage" :`true` "/Game/MultiplayerFPSEngine/Sword/AttackRight_Montage.AttackRight_Montage" :!type "AnimMontage Object Reference") 1.3 "None")
    (set `self.AttackDelay` 0.7)
    (set `self.attack` (not (`self.attack`)))
    (`KismetSystemLibrary.Delay` 0.1)
    (`GameplayStatics.PlaySound2D` null 1.0 1.0 0.0 null null)
    (`KismetSystemLibrary.Delay` 0.35)
    (`KismetSystemLibrary.CapsuleTraceSingle` _returnvalue (+ _returnvalue (* (`SceneComponent.GetForwardVector` _camera1) 150.0)) 20.0 20.0 "TraceTypeQuery1" false (`|MakeArray` (`self.player`) :!type "Actor Object Reference"))))

(event `self.ReceiveTick`
  (params (DeltaSeconds :type "Float (single-precision)"))
  (`parent.ReceiveTick` DeltaSeconds)
  (set `self.AttackDelay` (- (`self.AttackDelay`) DeltaSeconds)))

(fn `CalculateSpray`
  (returns (spray :type "Float (double-precision)"))
  (return -5.0))

(fn `UserConstructionScript`
  (`parent.UserConstructionScript`))